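; Interactable security camera screen for the tunnel security area, which starts black and acts as a keycard check.
; When a first-person character holding the keycard interacts, it switches once to the maintenance CCTV material and calls OpenGate on the inner security door.
; It binds to that door's action event, which sets the linked button's state and then unbinds itself.
; An outer door OpenGate call is left unconnected.
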(event Custom|MakeActiveButtons
  (params (GatesState :type EGatesAction%20Enum :default "NewEnumerator0"))
  (Default|SetState (Variables|Default|GetButton) "NewEnumerator0")
  (EventDispatchers|UnbindEventfromDoorAction (Variables|Default|GetSecurityDoorInner) (EventDispatchers|CreateEvent :!event Custom|MakeActiveButtons)))

(event EventInteracting
  (params (Interacter :type Pawn%20Object%20Reference))
  (bind _securitydoorinner (Variables|Default|GetSecurityDoorInner))
  (bind _asbp_first_person_char (Utilities|Casting|CastToBP_FirstPerson_Char Interacter))
  (if (Variables|/Game/SurvivalHorror/Assets/Characters/FirstPerson/Main/BP_FirstPerson_Char.BP_FirstPerson_Char_C|GetHaveKeyCard _asbp_first_person_char)
    (Utilities|FlowControl|DoOnce false
      (:Completed
        (Rendering|Material|SetMaterial (Variables|Default|GetScreen) 0 "/Game/SurvivalHorror/Maps/Parallel/Assets/Blueprints/Tunnel_Security/CCTV_MaintenanceCamera_Mat.CCTV_MaintenanceCamera_Mat")
        (Default|OpenGate _securitydoorinner "NewEnumerator0")
        (EventDispatchers|BindEventtoDoorAction _securitydoorinner (delegate Custom|MakeActiveButtons))))))

(event EventBeginPlay
  (|CallParentFunction)
  (Rendering|Material|SetMaterial (Variables|Default|GetScreen) 0 "/Engine/EngineDebugMaterials/BlackUnlitMaterial.BlackUnlitMaterial"))

(fn ConstructionScript)