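; Tunnel maintenance actor that unlocks a show-road cheat for toggling navigation arrows as a route hint.
; It gathers every BP_NavigationArrow at BeginPlay and permanently sets AllowCheat once BP_FirstPerson_Char overlaps its box.
; When unlocked, its HideArrows event loops over the arrows, with a FlipFlop inside the loop alternating the hide flag on each element.
; A second FlipFlop alternates printed show and hide hint messages per call.
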(event OnComponentBeginOverlap(Box)
  (params (OverlappedComponent :type Primitive%20Component%20Object%20Reference) (OtherActor :type Actor%20Object%20Reference) (OtherComp :type Primitive%20Component%20Object%20Reference) (OtherBodyIndex :type Integer) (bFromSweep :type Boolean) (SweepResult :type Hit%20Result%20Structure%20%28by%20ref%29))
  (Utilities|Casting|CastToBP_FirstPerson_Char OtherActor)
  (Variables|Default|SetAllowCheat true))

(event Custom|HideArrows
  (if (Variables|Default|GetAllowCheat)
    (for _array_element (Variables|Default|GetNavigationArrows)
      (Variables|Default|SetArray%20Element _array_element)
      (Utilities|FlowControl|FlipFlop
        (:A
          (Default|HideArrows (Variables|Default|GetArray%20Element) false))
        (:B
          (Default|HideArrows (Variables|Default|GetArray%20Element) true))))
    (Utilities|FlowControl|FlipFlop
      (:A
        (Development|PrintString "ShowRoadHint"))
      (:B
        (Development|PrintString "HideRoadHint")))))

(event EventBeginPlay
  (bind _outactors (Actor|GetAllActorsOfClass "/Game/SurvivalHorror/Maps/Parallel/Assets/Blueprints/Tunnel_Maintenance/BP_NavigationArrow.BP_NavigationArrow_C"))
  (Variables|Default|SetNavigationArrows _outactors))

(fn ConstructionScript)