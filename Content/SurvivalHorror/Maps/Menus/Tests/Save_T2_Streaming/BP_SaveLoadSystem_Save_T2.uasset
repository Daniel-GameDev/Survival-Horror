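; BP_SaveLoadSystem_Save_T2 is a test trigger volume that swaps streamed sublevels and saves player progress when the first-person character overlaps it.
; On overlap it captures the capsule transform, then blocking-loads and unloads the sublevels indexed from SubLevels.
; It creates the save slot if missing, then reloads it and writes the transform plus the player's level, unless that name is None.
; The construction script sizes the overlap box from a variable.
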(event OnComponentBeginOverlap(PlayerOverlapBox)
  (params (OverlappedComponent :type Primitive%20Component%20Object%20Reference) (OtherActor :type Actor%20Object%20Reference) (OtherComp :type Primitive%20Component%20Object%20Reference) (OtherBodyIndex :type Integer) (bFromSweep :type Boolean) (SweepResult :type Hit%20Result%20Structure%20%28by%20ref%29))
  (bind _sublevels (Variables|Default|GetSubLevels))
  (bind _levelofplayerposition (Variables|Default|GetLevelOfPlayerPosition))
  (bind _output (Utilities|Array|Get(acopy) _sublevels _levelofplayerposition))
  (bind _asbp_first_person_char (Utilities|Casting|CastToBP_FirstPerson_Char OtherActor))
  (Variables|Default|SetTransformToSave (Transformation|GetWorldTransform (Variables|/Script/Engine.Character|GetCapsuleComponent _asbp_first_person_char)))
  (Game|LoadStreamLevel(byName) (Utilities|Array|Get(acopy) (Variables|Default|GetSubLevels) (Variables|Default|GetLevelToLoad)) true true)
  (Game|UnloadStreamLevel(byName) (Utilities|Array|Get(acopy) (Variables|Default|GetSubLevels) (Variables|Default|GetLevelsToUnload)) true)
  (bind _returnvalue (SaveGame|DoesSaveGameExist "SaveSlot_Save_T2"))
  (if _returnvalue
    _
    (else
      (bind _returnvalue_2 (SaveGame|CreateSaveGameObject "/Game/SurvivalHorror/Maps/Menus/Tests/Save_T2_Streaming/SaveGame_Save_T2.SaveGame_Save_T2_C"))
      (SaveGame|SaveGametoSlot _returnvalue_2 "SaveSlot_Save_T2")
      (Utilities|FlowControl|Delay 0.2)))
  (bind _returnvalue_3 (SaveGame|LoadGamefromSlot "SaveSlot_Save_T2"))
  (bind _assave_game_save_t2 (Utilities|Casting|CastToSaveGame_Save_T2 _returnvalue_3))
  (if (not (Utilities|Name|Equal(Name) _output "None"))
    (Variables|/Game/SurvivalHorror/Maps/Menus/Tests/Save_T2_Streaming/SaveGame_Save_T2.SaveGame_Save_T2_C|SetCurrentLevel _assave_game_save_t2 _output))
  (Variables|/Game/SurvivalHorror/Maps/Menus/Tests/Save_T2_Streaming/SaveGame_Save_T2.SaveGame_Save_T2_C|SetPlayTransform _assave_game_save_t2 (Variables|Default|GetTransformToSave))
  (SaveGame|SaveGametoSlot _assave_game_save_t2 "SaveSlot_Save_T2"))

(fn ConstructionScript
  (Components|Box|SetBoxExtent (Variables|Default|GetPlayerOverlapBox) (Variables|Default|GetIn%20Box%20Extent) true))