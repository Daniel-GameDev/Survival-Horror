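; Security door for the tunnel map that slides vertically between open and closed positions, starting in its configured GatesState.
; OpenGate plays or reverses a timeline, scaled by TimeToComplete, that lerps the door's height.
; While closing, a box trace skips movement updates when something is in the doorway, though the timeline keeps running.
; On finish, it flips the state and broadcasts it through CallDoorAction.
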(event EventBeginPlay
  (bind _door (Variables|Default|GetDoor))
  (bind _door_2 (Variables|Default|GetDoor))
  (bind _relativelocation (Variables|/Script/Engine.SceneComponent|GetRelativeLocation _door))
  (bind _relativelocation_2 (Variables|/Script/Engine.SceneComponent|GetRelativeLocation _door_2))
  (Components|Timeline|SetPlayRate (Variables|Default|GetGatesOpenTime) (/ 1.0 (Variables|Default|GetTimeToComplete)))
  (switch Utilities|FlowControl|Switch|SwitchonEGatesAction (Variables|Default|GetGates%20State)
    (:NewEnumerator0
      (Variables|Default|SetGatesOpened true)
      (Transformation|SetRelativeLocation _door_2 (Math|Vector|MakeVector (.x _relativelocation_2) (.y _relativelocation_2) 4e+02) false false))
    (:NewEnumerator1
      (Variables|Default|SetGatesOpened false)
      (Transformation|SetRelativeLocation _door (Math|Vector|MakeVector (.x _relativelocation) (.y _relativelocation) 1e+02) false false))))

(event EventOpenGate
  (params (GatesAct :type EGatesAction%20Enum :default "NewEnumerator0"))
  (bind _door (Variables|Default|GetDoor))
  (bind _box (Variables|Default|GetBox))
  (bind (_origin _boxextent) (Collision|GetComponentBounds _box))
  (bind _relativelocation (Variables|/Script/Engine.SceneComponent|GetRelativeLocation _door))
  (switch Utilities|FlowControl|Switch|SwitchonEGatesAction GatesAct
    (:NewEnumerator0
      (if (not (Variables|Default|GetGatesOpened))
        (bind _openning (Timeline|GatesOpenTime Play)
          (:Update
            (if (Utilities|Enum|Equal(Enum) (Variables|Default|GetGates%20State) "NewEnumerator1")
              (Transformation|SetRelativeLocation _door (Math|Vector|MakeVector (.x _relativelocation) (.y _relativelocation) (Math|Float|Lerp 1e+02 4e+02 _openning)) false false :!label _label)
              (else
                (bind _returnvalue (Collision|BoxTraceByChannel _origin _origin _boxextent "0, 0, 0" "TraceTypeQuery1" false 0 "None" true "(R=1.000000,G=0.000000,B=0.000000,A=1.000000)" "(R=0.000000,G=0.614277,B=1.000000,A=1.000000)"))
                (if (not _returnvalue)
                  (goto _label)))))
          (:Finished
            (if (Variables|Default|GetGatesOpened)
              (Variables|Default|SetGatesOpened false)
              (Variables|Default|SetGates%20State "NewEnumerator1")
              (else
                (Variables|Default|SetGatesOpened true)
                (Variables|Default|SetGates%20State "NewEnumerator0")))
            (Default|CallDoorAction (Variables|Default|GetGates%20State))))))
    (:NewEnumerator1
      (if (Variables|Default|GetGatesOpened)
        (Timeline|GatesOpenTime Reverse)))))

(fn ConstructionScript)