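; Base pickup item for the InspectTest1 gym inventory, with a HUD prompt, pick up, drop and close-up inspection.
; Interacting attaches it to the player's grip, or starts inspection if the player already holds an item.
; Inspection shows a description widget and moves input to the item: gated left-mouse drag rotates it, the wheel sets camera distance, Interact exits.
; DropItem restores physics in front of the camera unless a trace is blocked.
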(event EventInteractwith
  (params (Player%20Char :type BP%20First%20Person%20Char%20Object%20Reference))
  (bind _output_get (Variables|Default|SetPlayer%20Char Player%20Char))
  (Variables|/Game/SurvivalHorror/Assets/Characters/FirstPerson/Main/BP_FirstPerson_Char.BP_FirstPerson_Char_C|GetCurrentlyHeldItem _output_get
    (:then
      (CallFunction|StartInspect))
    (:else
      (CallFunction|PickUpItem))))

(event EventLookat
  (params (PlayerChar :type BP%20First%20Person%20Char%20Object%20Reference))
  (bind _aswbp_hud_inspect_test_1 (Utilities|Casting|CastToWBP_HUD_InspectTest1 (Variables|/Game/SurvivalHorror/Assets/Characters/FirstPerson/Main/BP_FirstPerson_Char.BP_FirstPerson_Char_C|GetHUDWidget_InspectTest1 PlayerChar)))
  (Default|UpdateMessage _aswbp_hud_inspect_test_1 (Utilities|Text|FormatText "Press X to Pick Up {name}" (Variables|Default|GetItemName))))

(event Input|ActionEvents|InputActionInteract_InspectTest1
  (params (Key :type Key%20Structure :default "None"))
  (:Pressed
    (CallFunction|StopInspect)))

(event Input|MouseEvents|MouseX
  (params (AxisValue :type Float%20%28single-precision%29))
  (Utilities|FlowControl|Gate true
    (:Exit
      (Transformation|SetActorRotation (Math|Rotator|CombineRotators (Transformation|GetActorRotation) (Math|Rotator|MakeRotator 0.0 0.0 (* AxisValue -5.0)))))))

(event Input|MouseEvents|MouseY
  (params (AxisValue :type Float%20%28single-precision%29))
  (Utilities|FlowControl|Gate true
    (:Exit
      (Transformation|SetActorRotation (Math|Rotator|CombineRotators (Transformation|GetActorRotation) (Math|Rotator|MakeRotator 0.0 (* AxisValue -5.0) 0.0))))))

(event Input|MouseEvents|LeftMouseButton
  (params (Key :type Key%20Structure :default "None"))
  (:Pressed
    (Utilities|FlowControl|Sequence
      (:then_0
        (Utilities|FlowControl|Gate true) ; enters at Open
      )
      (:then_1
        (Utilities|FlowControl|Gate true) ; enters at Open
      )))
  (:Released
    (Utilities|FlowControl|Sequence
      (:then_0
        (Utilities|FlowControl|Gate true) ; enters at Close
      )
      (:then_1
        (Utilities|FlowControl|Gate true) ; enters at Close
      ))))

(event Input|MouseEvents|MouseWheelUp
  (params (Key :type Key%20Structure :default "None"))
  (bind _returnvalue (Game|GetPlayerCameraManager 0))
  ;[1 0.1039 0] FIXME: Очень дерганно
  (:Pressed
    (bind _output_get (Variables|Default|SetZoomLevel (Math|Integer|Clamp(Integer) (+ (Variables|Default|GetZoomLevel) 1) 1 20)))
    (if (< _output_get 10)
      (Transformation|SetActorLocation (+ (Camera|GetCameraLocation _returnvalue) (* (Transformation|GetActorForwardVector _returnvalue) (* (Variables|Default|GetZoomLevel) 2e+01))) false false))))

(event Input|MouseEvents|MouseWheelDown
  (params (Key :type Key%20Structure :default "None"))
  (bind _returnvalue (Game|GetPlayerCameraManager 0))
  ;[1 0.1039 0] FIXME: Очень дерганно
  (:Pressed
    (bind _output_get (Variables|Default|SetZoomLevel (Math|Integer|Clamp(Integer) (- (Variables|Default|GetZoomLevel) 1) 1 20)))
    (if (> _output_get 1)
      (Transformation|SetActorLocation (+ (Camera|GetCameraLocation _returnvalue) (* (Transformation|GetActorForwardVector _returnvalue) (* (Variables|Default|GetZoomLevel) 2e+01))) false false))))

(fn ConstructionScript)

(fn PickUpItem
  (bind _staticmesh (Variables|Default|GetStaticMesh))
  (Transformation|AttachComponentToComponent (Variables|/Game/SurvivalHorror/Assets/Characters/FirstPerson/Main/BP_FirstPerson_Char.BP_FirstPerson_Char_C|GetItemGrip%28InspectTest1%29 (Variables|Default|GetPlayer%20Char)) "None" "SnapToTarget" "SnapToTarget" "KeepRelative" true)
  (Physics|SetSimulatePhysics _staticmesh false)
  (Collision|SetCollisionEnabled _staticmesh "NoCollision")
  (Variables|/Game/SurvivalHorror/Assets/Characters/FirstPerson/Main/BP_FirstPerson_Char.BP_FirstPerson_Char_C|SetCurrentlyHeldItem (Variables|Default|GetPlayer%20Char) self))

(fn StartInspect
  (bind _returnvalue (Game|GetPlayerController 0))
  (bind _returnvalue_2 (Game|GetPlayerCameraManager 0))
  (Widget|SetVisibility (Variables|/Game/SurvivalHorror/Assets/Characters/FirstPerson/Main/BP_FirstPerson_Char.BP_FirstPerson_Char_C|GetHUDWidget_InspectTest1 (Variables|Default|GetPlayer%20Char)) "Hidden")
  (bind _returnvalue_3 (UserInterface|CreateWidget "/Game/SurvivalHorror/Assets/Characters/Widget/WBP_InspectionScreen_UI_InspectTest1.WBP_InspectionScreen_UI_InspectTest1_C" 0 (Variables|Default|GetItemDescription)))
  (bind _output_get (Variables|Default|SetInspectionUI _returnvalue_3))
  (UserInterface|Viewport|AddtoViewport _output_get 0)
  (Input|DisableInput (Variables|Default|GetPlayer%20Char) _returnvalue)
  (Input|EnableInput _returnvalue)
  (Transformation|SetActorLocation (+ (Camera|GetCameraLocation _returnvalue_2) (* (Transformation|GetActorForwardVector _returnvalue_2) 75.0)) false false))

(fn DropItem
  (bind _returnvalue (Game|GetPlayerCameraManager 0))
  (bind _staticmesh (Variables|Default|GetStaticMesh))
  (bind _returnvalue_2 (Camera|GetCameraLocation _returnvalue))
  (bind _returnvalue_3 (Transformation|GetActorForwardVector _returnvalue))
  (bind _returnvalue_4 (* _returnvalue_3 1e+02))
  (bind _returnvalue_5 (+ _returnvalue_2 _returnvalue_4))
  (bind _outhit (Collision|LineTraceByChannel _returnvalue_2 _returnvalue_5 "TraceTypeQuery2" false (Utilities|Array|MakeArray (Variables|Default|GetPlayer%20Char)) "None"))
  (if (.bblockinghit _outhit)
    (return false)
    (else
      (Transformation|DetachFromActor "KeepWorld" "KeepWorld" "KeepWorld")
      (Transformation|SetActorLocation _returnvalue_5 false false)
      (Physics|SetSimulatePhysics _staticmesh true)
      (Collision|SetCollisionEnabled _staticmesh "QueryAndPhysics")
      (return true))))

(fn StopInspect
  (bind _returnvalue (Game|GetPlayerController 0))
  (Input|DisableInput _returnvalue)
  (Input|EnableInput (Variables|Default|GetPlayer%20Char) _returnvalue)
  (Transformation|SetActorRelativeLocation "0, 0, 0")
  (Transformation|SetActorRelativeRotation "0, 0, 0")
  (bind _inspectionui (Variables|Default|GetInspectionUI)
    (:then
      (Widget|RemovefromParent _inspectionui)
      (Widget|SetVisibility (Variables|/Game/SurvivalHorror/Assets/Characters/FirstPerson/Main/BP_FirstPerson_Char.BP_FirstPerson_Char_C|GetHUDWidget_InspectTest1 (Variables|Default|GetPlayer%20Char)) "Visible"))
    (:else)))