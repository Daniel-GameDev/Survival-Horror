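; Experimental rope actor that builds a chain of capsule components along a Cable component's simulated particles.
; BeginPlay adds one capsule per particle location and makes it visible in game.
; Each Tick teleports every capsule to its particle and aligns it toward the next one, with the last using the direction from the previous capsule.
; Unconnected leftover nodes hold earlier sphere mesh and sphere component variants of the same approach.
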(event EventBeginPlay
  (for _array_element (Class|CableComponent|GetCableParticleLocations (Variables|Default|GetCable))
    (bind _returnvalue (AddComponent|AddCapsuleComponent false (Math|Transform|MakeTransform _array_element "0, 0, 0" (Variables|Default|GetSocket_RelativeTransformScale))))
    (Utilities|Array|Add (Variables|Default|GetCapsuleArray) _returnvalue)
    (Development|SetHiddeninGame _returnvalue false false)))

(event EventTick
  (params (DeltaSeconds :type Float%20%28single-precision%29))
  (bind _capsulearray (Variables|Default|GetCapsuleArray))
  (for (_array_element _array_index) (Class|CableComponent|GetCableParticleLocations (Variables|Default|GetCable))
    (Transformation|SetWorldLocation (Utilities|Array|Get(acopy) _capsulearray _array_index) _array_element false true)
    (Utilities|IsValid (Utilities|Array|Get(acopy) _capsulearray (+ _array_index 1))
      (:Is%20Valid
        (Transformation|SetWorldRotation (Utilities|Array|Get(acopy) _capsulearray _array_index) (Math|Rotator|MakeRotator 0.0 (+ (.pitch (Math|Rotator|FindLookatRotation (Transformation|GetWorldLocation (Utilities|Array|Get(acopy) _capsulearray _array_index)) (Transformation|GetWorldLocation (Utilities|Array|Get(acopy) _capsulearray (+ _array_index 1))))) 9e+01) (.yaw (Math|Rotator|FindLookatRotation (Transformation|GetWorldLocation (Utilities|Array|Get(acopy) _capsulearray _array_index)) (Transformation|GetWorldLocation (Utilities|Array|Get(acopy) _capsulearray (+ _array_index 1)))))) false true))
      (:Is%20Not%20Valid
        (Utilities|IsValid (Utilities|Array|Get(acopy) (Variables|Default|GetCapsuleArray) (- _array_index 1))
          (:Is%20Valid
            (Transformation|SetWorldRotation (Utilities|Array|Get(acopy) _capsulearray _array_index) (Math|Rotator|MakeRotator 0.0 (+ (.pitch (Math|Rotator|FindLookatRotation (Transformation|GetWorldLocation (Utilities|Array|Get(acopy) (Variables|Default|GetCapsuleArray) (- _array_index 1))) (Transformation|GetWorldLocation (Utilities|Array|Get(acopy) _capsulearray _array_index)))) 9e+01) (.yaw (Math|Rotator|FindLookatRotation (Transformation|GetWorldLocation (Utilities|Array|Get(acopy) (Variables|Default|GetCapsuleArray) (- _array_index 1))) (Transformation|GetWorldLocation (Utilities|Array|Get(acopy) _capsulearray _array_index))))) false true)))))))

(fn ConstructionScript)