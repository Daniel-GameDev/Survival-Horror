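; Experimental rope actor that gives a hanging Cable component collision-style capsules that follow its simulation.
; The construction script traces down to size the cable above the floor, only printing "Delete" when space is too short.
; BeginPlay spawns a visible capsule per cable particle, and Tick teleports each onto its particle, aligned along the neighbouring segment.
; A TODO notes the missing half-segment offset, and an unused trace copy remains in EventGraph.
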(event EventBeginPlay
  (for _array_element (Class|CableComponent|GetCableParticleLocations (Variables|Default|GetCable))
    (bind _returnvalue (AddComponent|AddCapsuleComponent false (Math|Transform|MakeTransform _array_element "0, 0, 0" (Variables|Default|GetSocket_RelativeTransformScale))))
    (Utilities|Array|Add (Variables|Default|GetCapsuleArray) _returnvalue)
    (Development|SetHiddeninGame _returnvalue false false)))

(event EventTick
  (params (DeltaSeconds :type Float%20%28single-precision%29))
  (bind _capsulearray (Variables|Default|GetCapsuleArray))
  ;[0 0.6143 1] TODO: расстояние между фиксированными партиклами / 2 и есть нужное мне расстояние которое нужно отнимать в установке локации для капусль колизий - нужно получить расстояние между фиксированными партиклами, поделить его на 2, прибавить это значения к локации апдейта капсул коллизии
  (for (_array_element _array_index) (Class|CableComponent|GetCableParticleLocations (Variables|Default|GetCable))
    (Transformation|SetWorldLocation (Utilities|Array|Get(acopy) _capsulearray _array_index) _array_element false true)
    (Utilities|IsValid (Utilities|Array|Get(acopy) _capsulearray (+ _array_index 1))
      (:Is%20Valid
        (Transformation|SetWorldRotation (Utilities|Array|Get(acopy) _capsulearray _array_index) (Math|Rotator|MakeRotator 0.0 (+ (.pitch (Math|Rotator|FindLookatRotation (Transformation|GetWorldLocation (Utilities|Array|Get(acopy) _capsulearray _array_index)) (Transformation|GetWorldLocation (Utilities|Array|Get(acopy) _capsulearray (+ _array_index 1))))) 9e+01) (.yaw (Math|Rotator|FindLookatRotation (Transformation|GetWorldLocation (Utilities|Array|Get(acopy) _capsulearray _array_index)) (Transformation|GetWorldLocation (Utilities|Array|Get(acopy) _capsulearray (+ _array_index 1)))))) false true))
      (:Is%20Not%20Valid
        (Utilities|IsValid (Utilities|Array|Get(acopy) (Variables|Default|GetCapsuleArray) (- _array_index 1))
          (:Is%20Valid
            (Transformation|SetWorldRotation (Utilities|Array|Get(acopy) _capsulearray _array_index) (Math|Rotator|MakeRotator 0.0 (+ (.pitch (Math|Rotator|FindLookatRotation (Transformation|GetWorldLocation (Utilities|Array|Get(acopy) (Variables|Default|GetCapsuleArray) (- _array_index 1))) (Transformation|GetWorldLocation (Utilities|Array|Get(acopy) _capsulearray _array_index)))) 9e+01) (.yaw (Math|Rotator|FindLookatRotation (Transformation|GetWorldLocation (Utilities|Array|Get(acopy) (Variables|Default|GetCapsuleArray) (- _array_index 1))) (Transformation|GetWorldLocation (Utilities|Array|Get(acopy) _capsulearray _array_index))))) false true)))))))

(fn ConstructionScript
  (bind _cable (Variables|Default|GetCable))
  (bind _returnvalue (Transformation|GetWorldLocation _cable))
  (bind (_x _y _z) (Math|Vector|BreakVector _returnvalue))
  (bind (_outhit _returnvalue_2) (Collision|LineTraceByChannel _returnvalue (Math|Vector|MakeVector _x _y (- _z (Variables|Default|GetTraceCableLength))) "TraceTypeQuery1" false 0 "ForDuration" true "(R=1.000000,G=0.000000,B=0.000000,A=1.000000)" "(R=0.000000,G=1.000000,B=0.000000,A=1.000000)" 1e+01))
  (if _returnvalue_2
    (if (< (- (.Distance (Collision|BreakHitResult _outhit)) (Variables|Default|GetFloorSpacerLength)) 2e+02)
      (Development|PrintString "Delete")
      (else
        (Variables|/Script/CableComponent.CableComponent|SetCableLength (Variables|Default|GetCable) (- (.Distance (Collision|BreakHitResult _outhit)) (Variables|Default|GetFloorSpacerLength)))))
    (else
      (Variables|/Script/CableComponent.CableComponent|SetCableLength (Variables|Default|GetCable) (- (Variables|Default|GetTraceCableLength) (Variables|Default|GetFloorSpacerLength))))))