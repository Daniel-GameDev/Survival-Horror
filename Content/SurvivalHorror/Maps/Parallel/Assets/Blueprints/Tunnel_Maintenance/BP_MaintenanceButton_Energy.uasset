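; Interactable maintenance-tunnel button that toggles its linked gates open and closed, tied to an energy box's power event.
; Its Active, Disable or Broken state drives interactivity, glow material and spotlight, with EnergyOn switching it to Active.
; A press animates the button via timeline, dims it and sends alternating Open/Close to each door.
; A DoOnce blocks presses until doors report Open or Close; Half shows the button broken.
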(event Custom|DoorOpened_Event_0
  (params (GatesState :type EGatesAction%20Enum :default "NewEnumerator0"))
  (bind _button (Variables|Default|GetButton))
  (bind _relativelocation (Variables|/Script/Engine.SceneComponent|GetRelativeLocation _button))
  (switch Utilities|FlowControl|Switch|SwitchonEGatesAction GatesState
    (:NewEnumerator0
      (Development|PrintString (Utilities|String|EnumtoString GatesState) :!label _label)
      (Utilities|FlowControl|Sequence
        (:then_0
          (Rendering|Material|SetVectorParameterValue (Variables|Default|GetButtonMaterial) "GlowTint" (Variables|Default|GetActiveColor) :!class /Script/Engine.MaterialInstanceDynamic)
          (Rendering|Components|Light|SetLightColor (Variables|Default|GetSpotLight) (Variables|Default|GetActiveColor) true))
        (:then_1
          (Utilities|FlowControl|DoOnce false) ; enters at Reset
        )))
    (:NewEnumerator1
      (goto _label))
    (:NewEnumerator2
      (Rendering|Material|SetMaterial (Variables|Default|GetButton) 0 "/Engine/BasicShapes/BasicShapeMaterial.BasicShapeMaterial")
      (Components|DestroyComponent (Variables|Default|GetSpotLight)))))

(event Custom|EnergyOn
  (Variables|Default|SetButtonState "NewEnumerator0")
  (switch Utilities|FlowControl|Switch|SwitchonEButtonState (Variables|Default|GetButtonState)
    (:NewEnumerator0
      (Variables|Default|SetDisableButton%28Temp-NeedToUpdatedInteractbleObject%29 false)
      (Rendering|Material|SetMaterial (Variables|Default|GetButton) 0 (Variables|Default|GetButtonMaterial))
      (Rendering|Material|SetVectorParameterValue (Variables|Default|GetButtonMaterial) "GlowTint" (Variables|Default|GetActiveColor) :!class /Script/Engine.MaterialInstanceDynamic)
      (Rendering|Components|Light|SetLightColor (Variables|Default|GetSpotLight) (Variables|Default|GetActiveColor) true)
      (Development|SetHiddeninGame (Variables|Default|GetSpotLight) false false))
    (:NewEnumerator1
      (Variables|Default|SetDisableButton%28Temp-NeedToUpdatedInteractbleObject%29 true)
      (Rendering|Material|SetVectorParameterValue (Variables|Default|GetButtonMaterial) "GlowTint" (Variables|Default|GetDisableColor) :!class /Script/Engine.MaterialInstanceDynamic)
      (Rendering|Components|Light|SetLightColor (Variables|Default|GetSpotLight) (Variables|Default|GetDisableColor) true))
    (:NewEnumerator2
      (Variables|Default|SetDisableButton%28Temp-NeedToUpdatedInteractbleObject%29 true)
      (Rendering|Material|SetMaterial (Variables|Default|GetButton) 0 "/Engine/BasicShapes/BasicShapeMaterial.BasicShapeMaterial")
      (Development|SetHiddeninGame (Variables|Default|GetSpotLight) true false))))

(event EventInteracting
  (params (Interacter :type Pawn%20Object%20Reference))
  (bind _button (Variables|Default|GetButton))
  (bind _relativelocation (Variables|/Script/Engine.SceneComponent|GetRelativeLocation _button))
  (if (not (Variables|Default|GetDisableButton%28Temp-NeedToUpdatedInteractbleObject%29))
    (Utilities|FlowControl|DoOnce false
      (:Completed
        (Utilities|FlowControl|FlipFlop
          (:A
            (Variables|Default|SetGates%20Act "NewEnumerator0"))
          (:B
            (Variables|Default|SetGates%20Act "NewEnumerator1")))
        (Default|CallPressed)
        (bind _pressing (Timeline|ButtonPressTime PlayFromStart)
          (:Update
            (Transformation|SetRelativeLocation _button (Math|Vector|MakeVector (Math|Float|Lerp -8e+01 -83.0 _pressing) (.y _relativelocation) (.z _relativelocation)) false false))
          (:Finished
            (Utilities|FlowControl|Sequence
              (:then_0
                (Rendering|Material|SetVectorParameterValue (Variables|Default|GetButtonMaterial) "GlowTint" (Variables|Default|GetDisableColor) :!class /Script/Engine.MaterialInstanceDynamic)
                (Rendering|Components|Light|SetLightColor (Variables|Default|GetSpotLight) (Variables|Default|GetDisableColor) true))
              (:then_1
                (for _array_element (Variables|Default|GetDoors)
                  (Default|OpenGate _array_element (Variables|Default|GetGates%20Act)))))))))))

(event EventBeginPlay
  (|CallParentFunction)
  (EventDispatchers|BindEventtoGotEnergy (Variables|Default|GetEnergyBox) (EventDispatchers|CreateEvent :!event Custom|EnergyOn))
  (for _array_element (Variables|Default|GetDoors)
    (EventDispatchers|AssignDoorAction _array_element (EventDispatchers|CreateEvent :!event Custom|DoorOpened_Event_0))
    (switch Utilities|FlowControl|Switch|SwitchonEButtonState (Variables|Default|GetButtonState)
      (:NewEnumerator0
        (Variables|Default|SetDisableButton%28Temp-NeedToUpdatedInteractbleObject%29 false)
        (Rendering|Material|SetMaterial (Variables|Default|GetButton) 0 (Variables|Default|GetButtonMaterial))
        (Rendering|Material|SetVectorParameterValue (Variables|Default|GetButtonMaterial) "GlowTint" (Variables|Default|GetActiveColor) :!class /Script/Engine.MaterialInstanceDynamic)
        (Rendering|Components|Light|SetLightColor (Variables|Default|GetSpotLight) (Variables|Default|GetActiveColor) true)
        (Development|SetHiddeninGame (Variables|Default|GetSpotLight) false false))
      (:NewEnumerator1
        (Variables|Default|SetDisableButton%28Temp-NeedToUpdatedInteractbleObject%29 true)
        (Rendering|Material|SetVectorParameterValue (Variables|Default|GetButtonMaterial) "GlowTint" (Variables|Default|GetDisableColor) :!class /Script/Engine.MaterialInstanceDynamic)
        (Rendering|Components|Light|SetLightColor (Variables|Default|GetSpotLight) (Variables|Default|GetDisableColor) true))
      (:NewEnumerator2
        (Variables|Default|SetDisableButton%28Temp-NeedToUpdatedInteractbleObject%29 true)
        (Rendering|Material|SetMaterial (Variables|Default|GetButton) 0 "/Engine/BasicShapes/BasicShapeMaterial.BasicShapeMaterial")
        (Development|SetHiddeninGame (Variables|Default|GetSpotLight) true false)))))

(fn ConstructionScript
  (bind _returnvalue (Rendering|Material|CreateDynamicMaterialInstance (Variables|Default|GetButton) 0 "/Game/SurvivalHorror/Maps/Parallel/Assets/Materials/M_Glow_Inst_Button.M_Glow_Inst_Button" "None" :!class /Script/Engine.PrimitiveComponent))
  (Variables|Default|SetButtonMaterial _returnvalue)
  (switch Utilities|FlowControl|Switch|SwitchonEButtonState (Variables|Default|GetButtonState)
    (:NewEnumerator0
      (Rendering|Material|SetVectorParameterValue (Variables|Default|GetButtonMaterial) "GlowTint" (Variables|Default|GetActiveColor) :!class /Script/Engine.MaterialInstanceDynamic)
      (Rendering|Components|Light|SetLightColor (Variables|Default|GetSpotLight) (Variables|Default|GetActiveColor) true))
    (:NewEnumerator1
      (Rendering|Material|SetVectorParameterValue (Variables|Default|GetButtonMaterial) "GlowTint" (Variables|Default|GetDisableColor) :!class /Script/Engine.MaterialInstanceDynamic)
      (Rendering|Components|Light|SetLightColor (Variables|Default|GetSpotLight) (Variables|Default|GetDisableColor) true))))