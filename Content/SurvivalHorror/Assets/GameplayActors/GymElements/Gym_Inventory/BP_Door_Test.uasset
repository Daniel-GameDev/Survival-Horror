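; Test door for the inventory gym that opens only when the player holds its matching key item.
; On look-at it updates the player's inspect HUD with either an open prompt naming the held item or a hint to find the key.
; On interact with the correct key it plays a timeline that yaws the door mesh open, then destroys the held key actor.
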(event Custom|OpenDoor
  (bind _dooropentrack (Timeline|DoorPosition Play)
    (:Update
      (Transformation|SetRelativeRotation (Variables|Default|GetDoor) (Math|Rotator|MakeRotator 0.0 0.0 _dooropentrack) false false))))

(event EventLookat
  (params (PlayerChar :type BP%20First%20Person%20Char%20Object%20Reference))
  (bind _hudwidget_inspecttest1 (Variables|/Game/SurvivalHorror/Assets/Characters/FirstPerson/Main/BP_FirstPerson_Char.BP_FirstPerson_Char_C|GetHUDWidget_InspectTest1 PlayerChar))
  (bind _currentlyhelditem (Variables|/Game/SurvivalHorror/Assets/Characters/FirstPerson/Main/BP_FirstPerson_Char.BP_FirstPerson_Char_C|GetCurrentlyHeldItem PlayerChar))
  (if (== _currentlyhelditem (Variables|Components|GetKey))
    (bind _aswbp_hud_inspect_test_1 (Utilities|Casting|CastToWBP_HUD_InspectTest1 _hudwidget_inspecttest1))
    (Default|UpdateMessage _aswbp_hud_inspect_test_1 (Utilities|Text|FormatText "Press X to Open Door with {name}" (Variables|/Game/SurvivalHorror/Assets/GameplayActors/GymElements/Gym_Inventory/Items_InspectTest1/BP_ItemParent_InspectTest1.BP_ItemParent_InspectTest1_C|GetItemName _currentlyhelditem)))
    (else
      (bind _aswbp_hud_inspect_test_1_2 (Utilities|Casting|CastToWBP_HUD_InspectTest1 _hudwidget_inspecttest1))
      (Default|UpdateMessage _aswbp_hud_inspect_test_1_2 "Find the Key to Open the Door"))))

(event EventInteractwith
  (params (Player%20Char :type BP%20First%20Person%20Char%20Object%20Reference))
  (bind _currentlyhelditem (Variables|/Game/SurvivalHorror/Assets/Characters/FirstPerson/Main/BP_FirstPerson_Char.BP_FirstPerson_Char_C|GetCurrentlyHeldItem Player%20Char))
  (if (== _currentlyhelditem (Variables|Components|GetKey))
    (CallFunction|OpenDoor)
    (Actor|DestroyActor _currentlyhelditem)))

(fn ConstructionScript)