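; BP_GasZone is a hazard volume that damages the overlapping actor with gas over time.
; Box overlap events set a shared overlap flag for any actor and toggle TakingGasDamage on the first-person character.
; The character's entry starts a looping half-second timer that applies gas-typed damage to the overlap event's actor while the flag is true.
; Each hit re-sets the timer, and exit only clears flags; EnterGasZone is empty.
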(event OnComponentBeginOverlap(Box)
  (params (OverlappedComponent :type Primitive%20Component%20Object%20Reference) (OtherActor :type Actor%20Object%20Reference) (OtherComp :type Primitive%20Component%20Object%20Reference) (OtherBodyIndex :type Integer) (bFromSweep :type Boolean) (SweepResult :type Hit%20Result%20Structure%20%28by%20ref%29))
  ;[1 0.465 0] OPTIMIZE: Change Cast to something else
  (Variables|Default|SetActorOverlaping true)
  (bind _asbp_first_person_char (Utilities|Casting|CastToBP_FirstPerson_Char OtherActor))
  (Variables|/Game/SurvivalHorror/Assets/Characters/FirstPerson/Main/BP_FirstPerson_Char.BP_FirstPerson_Char_C|SetTakingGasDamage _asbp_first_person_char true)
  (Utilities|Time|SetTimerbyEvent (delegate Custom|ApplyGasDamage) 0.5 true))

(event OnComponentEndOverlap(Box)
  (params (OverlappedComponent :type Primitive%20Component%20Object%20Reference) (OtherActor :type Actor%20Object%20Reference) (OtherComp :type Primitive%20Component%20Object%20Reference) (OtherBodyIndex :type Integer))
  ;[1 0.465 0] OPTIMIZE: Change Cast to something else
  (Variables|Default|SetActorOverlaping false)
  (bind _asbp_first_person_char (Utilities|Casting|CastToBP_FirstPerson_Char OtherActor))
  (Variables|/Game/SurvivalHorror/Assets/Characters/FirstPerson/Main/BP_FirstPerson_Char.BP_FirstPerson_Char_C|SetTakingGasDamage _asbp_first_person_char false))

(event Custom|ApplyGasDamage
  ;[1 0.465 0] OPTIMIZE: Change Cast to something else
  (if (Variables|Default|GetActorOverlaping)
    (Game|Damage|ApplyDamage (stale OnComponentBeginOverlap(Box) OtherActor) 1.0 0 self "/Game/SurvivalHorror/Assets/Characters/DamageType/DmgType_Gas.DmgType_Gas_C")
    (Utilities|Time|SetTimerbyEvent (delegate Custom|ApplyGasDamage) 0.5 true)))

(event EventBeginPlay)

(event Collision|EventActorBeginOverlap
  (params (OtherActor :type Actor%20Object%20Reference)))

(event EventTick
  (params (DeltaSeconds :type Float%20%28single-precision%29)))

(fn ConstructionScript)

(fn EnterGasZone)