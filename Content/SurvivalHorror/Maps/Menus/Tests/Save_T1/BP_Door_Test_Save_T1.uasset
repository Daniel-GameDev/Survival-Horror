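; Test door for a save-system test map that swings open when the first-person character enters its box trigger and never closes.
; If not already open, a timeline drives the door's yaw, then sets the Open flag and reports the door to GameState_Save_T1.
; BeginPlay and UpdateDoor share a check that snaps an already-open door to its open rotation, allowing its state to be reapplied without animation.
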(event OnComponentBeginOverlap(Box)
  (params (OverlappedComponent :type Primitive%20Component%20Object%20Reference) (OtherActor :type Actor%20Object%20Reference) (OtherComp :type Primitive%20Component%20Object%20Reference) (OtherBodyIndex :type Integer) (bFromSweep :type Boolean) (SweepResult :type Hit%20Result%20Structure%20%28by%20ref%29))
  (Utilities|Casting|CastToBP_FirstPerson_Char OtherActor)
  (CallFunction|OpenDoor))

(event Custom|OpenDoor
  (if (not (Variables|Default|GetbOpen))
    (bind _dooropentrack (Timeline|DoorPosition Play)
      (:Update
        (Transformation|SetRelativeRotation (Variables|Default|GetDoor) (Math|Rotator|MakeRotator 0.0 0.0 _dooropentrack) false false))
      (:Finished
        (Variables|Default|SetbOpen true)
        (bind _asgame_state_save_t1 (Utilities|Casting|CastToGameState_Save_T1 (Game|GetGameState)))
        (Default|CallDoorOpened _asgame_state_save_t1 self)))))

(event Custom|UpdateDoor
  (if (Variables|Default|GetbOpen)
    (Transformation|SetRelativeRotation (Variables|Default|GetDoor) (Math|Rotator|MakeRotator 0.0 0.0 9e+01) false false)))

(event EventBeginPlay
  (if (Variables|Default|GetbOpen)
    (Transformation|SetRelativeRotation (Variables|Default|GetDoor) (Math|Rotator|MakeRotator 0.0 0.0 9e+01) false false)))

(fn ConstructionScript)