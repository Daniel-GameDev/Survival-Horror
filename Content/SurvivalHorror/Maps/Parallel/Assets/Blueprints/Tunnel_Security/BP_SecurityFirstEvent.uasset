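; Scripted one-time event that puts the tunnel security area into alert, opening half and full doors.
; BeginPlay gathers light actors by class, binds TriggerButton's press, then also fires the event immediately.
; A DoOnce-guarded handler opens the gates, disables the button and switches off security lights.
; It also reveals warning lights and turns tunnel lights red at half intensity with alert glow materials.
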(event Custom|Pressed_Event_0
  (Utilities|FlowControl|DoOnce false
    (:Completed
      (for _array_element (Variables|Default|GetHalfDoors)
        (Default|OpenGate _array_element "NewEnumerator2")
        (Variables|/Game/SurvivalHorror/Maps/Parallel/Assets/Blueprints/Tunnel_Security/BP_SecurityButton.BP_SecurityButton_C|SetDisableButton%28Temp-NeedToUpdatedInteractbleObject%29 (Variables|Default|GetTriggerButton) true))
      (for _array_element_2 (Variables|Default|GetFullDoors)
        (Default|OpenGate _array_element_2 "NewEnumerator0"))
      (for _array_element_3 (Variables|Default|GetSecurityMainLights)
        (Rendering|SetVisibility (Variables|/Game/SurvivalHorror/Maps/Parallel/Assets/Blueprints/Tunnel_Security/BP_Security_MainLight.BP_Security_MainLight_C|GetPointLight _array_element_3) false false)
        (Rendering|Material|SetMaterial (Variables|/Game/SurvivalHorror/Maps/Parallel/Assets/Blueprints/Tunnel_Security/BP_Security_MainLight.BP_Security_MainLight_C|GetStaticMesh _array_element_3) 0 "/Engine/BasicShapes/BasicShapeMaterial.BasicShapeMaterial"))
      (for _array_element_4 (Variables|Default|GetSecuritySpotLight)
        (Rendering|SetVisibility (Variables|/Game/SurvivalHorror/Maps/Parallel/Assets/Blueprints/Tunnel_Security/BP_Security_SpotLight.BP_Security_SpotLight_C|GetSpotLight _array_element_4) false false)
        (Rendering|Material|SetMaterial (Variables|/Game/SurvivalHorror/Maps/Parallel/Assets/Blueprints/Tunnel_Security/BP_Security_SpotLight.BP_Security_SpotLight_C|GetStaticMesh _array_element_4) 0 "/Engine/BasicShapes/BasicShapeMaterial.BasicShapeMaterial"))
      (for _array_element_5 (Variables|Default|GetTunnelSpotLight)
        (Rendering|Components|Light|SetIntensity (Variables|/Game/SurvivalHorror/Maps/Parallel/Assets/Blueprints/Tunnel/BP_Tunnel_SpotLight.BP_Tunnel_SpotLight_C|GetSpotLight _array_element_5) (/ (Variables|/Script/Engine.LightComponentBase|GetIntensity (Variables|/Game/SurvivalHorror/Maps/Parallel/Assets/Blueprints/Tunnel/BP_Tunnel_SpotLight.BP_Tunnel_SpotLight_C|GetSpotLight _array_element_5)) 2.0))
        (Rendering|Components|Light|SetLightColor (Variables|/Game/SurvivalHorror/Maps/Parallel/Assets/Blueprints/Tunnel/BP_Tunnel_SpotLight.BP_Tunnel_SpotLight_C|GetSpotLight _array_element_5) "(R=1.000000,G=0.103898,B=0.000000,A=1.000000)" true)
        (Rendering|Material|SetMaterial (Variables|/Game/SurvivalHorror/Maps/Parallel/Assets/Blueprints/Tunnel/BP_Tunnel_SpotLight.BP_Tunnel_SpotLight_C|GetStaticMesh _array_element_5) 0 "/Game/SurvivalHorror/Maps/Parallel/Assets/Materials/M_Glow_Inst_Alert.M_Glow_Inst_Alert"))
      (for _array_element_6 (Variables|Default|GetWarningLight)
        (Rendering|SetActorHiddenInGame _array_element_6 false))
      (for _array_element_7 (Variables|Default|GetTunnelMainLight)
        (Rendering|Components|Light|SetIntensity (Variables|/Game/SurvivalHorror/Maps/Parallel/Assets/Blueprints/Tunnel/BP_Tunnel_MainLight.BP_Tunnel_MainLight_C|GetPointLight _array_element_7) (/ (Variables|/Script/Engine.LightComponentBase|GetIntensity (Variables|/Game/SurvivalHorror/Maps/Parallel/Assets/Blueprints/Tunnel/BP_Tunnel_MainLight.BP_Tunnel_MainLight_C|GetPointLight _array_element_7)) 2.0))
        (Rendering|Components|Light|SetLightColor (Variables|/Game/SurvivalHorror/Maps/Parallel/Assets/Blueprints/Tunnel/BP_Tunnel_MainLight.BP_Tunnel_MainLight_C|GetPointLight _array_element_7) "(R=1.000000,G=0.000000,B=0.000000,A=1.000000)" true)
        (Rendering|Material|SetMaterial (Variables|/Game/SurvivalHorror/Maps/Parallel/Assets/Blueprints/Tunnel/BP_Tunnel_MainLight.BP_Tunnel_MainLight_C|GetStaticMesh _array_element_7) 0 "/Game/SurvivalHorror/Maps/Parallel/Assets/Materials/M_Glow_Inst_Alert.M_Glow_Inst_Alert")))))

(event EventBeginPlay
  (EventDispatchers|AssignPressed (Variables|Default|GetTriggerButton) (delegate Custom|Pressed_Event_0))
  (bind _outactors (Actor|GetAllActorsOfClass "/Game/SurvivalHorror/Maps/Parallel/Assets/Blueprints/Tunnel_Security/BP_Security_MainLight.BP_Security_MainLight_C"))
  (Variables|Default|SetSecurityMainLights _outactors)
  (bind _outactors_2 (Actor|GetAllActorsOfClass "/Game/SurvivalHorror/Maps/Parallel/Assets/Blueprints/Tunnel/BP_Tunnel_SpotLight.BP_Tunnel_SpotLight_C"))
  (Variables|Default|SetTunnelSpotLight _outactors_2)
  (bind _outactors_3 (Actor|GetAllActorsOfClass "/Game/SurvivalHorror/Maps/Parallel/Assets/Blueprints/Tunnel_Security/BP_Security_WarningLight.BP_Security_WarningLight_C"))
  (Variables|Default|SetWarningLight _outactors_3)
  (bind _outactors_4 (Actor|GetAllActorsOfClass "/Game/SurvivalHorror/Maps/Parallel/Assets/Blueprints/Tunnel/BP_Tunnel_MainLight.BP_Tunnel_MainLight_C"))
  (Variables|Default|SetTunnelMainLight _outactors_4)
  (CallFunction|PressedEvent0))

(fn ConstructionScript)