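; Inventory component that holds item ID and quantity pairs in a fixed slot array, sized on BeginPlay when owned by BP_FirstPerson_Char, with extra hand slots unless flagged as a container.
; AddItem fills the first empty slot with quantity one, without stacking, or shows the WBP_NoSpace widget when full.
; Helpers swap the camera's post-process settings and set the left-hand mesh from DT_ItemData, though AddItem's hand check is disconnected.
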(event Custom|PrintInventory
  (for _array_element (Variables|Default|GetContent)
    (Development|PrintString (Utilities|String|ToString(Name) (.itemid _array_element)))
    (Development|PrintString (Utilities|String|ToString(Integer) (.quantity _array_element)))))

(event EventBeginPlay
  (bind _asbp_first_person_char (Utilities|Casting|CastToBP_FirstPerson_Char (Components|GetOwner)))
  (Variables|Default|SetAs%20BP%20First%20Person%20Char _asbp_first_person_char)
  (if (Variables|Default|GetContainer)
    (Utilities|Array|Resize (Variables|Default|GetContent) (Variables|Default|GetInventorySlots))
    (else
      (Utilities|Array|Resize (Variables|Default|GetContent) (+ (Variables|Default|GetInventorySlots) (Variables|Default|GetHands))))))

(fn FindEmptySlot
  (params (ItemId :type Name))
  (for (_array_element _array_index) (Variables|Default|GetContent)
    (if (Utilities|Name|Equal(Name) (.itemid _array_element) "None")
      (bind _output_get (LocalVariables|SetLocal_HasEmptySlot true))
      (return _output_get _array_index)))
  (bind _output_get_2 (LocalVariables|SetLocal_HasEmptySlot false))
  (return _output_get_2 -1))

(fn AddtoInventory
  (params (ItemId :type Name) (Index :type Integer))
  (Utilities|Array|SetArrayElem (Variables|Default|GetContent) Index (Utilities|Struct|MakeSItemStruct ItemId 1)))

(fn AddItem
  (params (ItemId :type Name))
  (bind (_hasemptyslot _index) (CallFunction|FindEmptySlot ItemId))
  (if _hasemptyslot
    (CallFunction|AddtoInventory ItemId _index)
    (if (Variables|Default|GetContainer)
      (return true)
      (else
        (return true)))
    (else
      (Development|PrintString "NoFreeSlots")
      (CallFunction|NoFreeSlots)
      (return false))))

(fn NoFreeSlots
  (bind _returnvalue (UserInterface|CreateWidget "/Game/SurvivalHorror/Assets/GameplayActors/GymElements/Common/Widgets/WBP_NoSpace.WBP_NoSpace_C" (Game|GetPlayerController 0)))
  (UserInterface|Viewport|AddtoViewport _returnvalue 0))

(fn PostProcces
  (params (Enable :type Boolean))
  (Variables|Default|GetFirst%20Person%20Camera
    (:then
      _)
    (:else
      (bind _output_get (Variables|Default|SetFirst%20Person%20Camera (Variables|/Game/SurvivalHorror/Assets/Characters/FirstPerson/Main/BP_FirstPerson_Char.BP_FirstPerson_Char_C|GetFirstPersonCamera (Variables|Default|GetAs%20BP%20First%20Person%20Char))))))
  (if Enable
    (Variables|Default|SetPostProcessSave (Variables|/Script/Engine.CameraComponent|GetPostProcessSettings _output_get))
    (Variables|/Script/Engine.CameraComponent|SetPostProcessSettings (Variables|Default|GetFirst%20Person%20Camera) (Variables|Default|GetPostProcess))
    (Class|CameraComponent|SetPostProcessBlendWeight (Variables|Default|GetFirst%20Person%20Camera) 1.0)
    (else
      (Variables|/Script/Engine.CameraComponent|SetPostProcessSettings (Variables|Default|GetFirst%20Person%20Camera) (Variables|Default|GetPostProcessSave))
      (Class|CameraComponent|SetPostProcessBlendWeight (Variables|Default|GetFirst%20Person%20Camera) 0.0))))

(fn CheckIteminHands
  (params (Index :type Integer) (ItemId :type Name))
  (if (== Index 0)
    (bind _returnvalue (Utilities|GetDataTableRow "/Game/SurvivalHorror/Assets/GameplayActors/GymElements/Gym_Inventory/CustomInventory/DT_ItemData.DT_ItemData" ItemId)
      (:then
        (Components|StaticMesh|SetStaticMesh (Variables|/Game/SurvivalHorror/Assets/Characters/FirstPerson/Main/BP_FirstPerson_Char.BP_FirstPerson_Char_C|GetLeftHandMesh (Variables|Default|GetAs%20BP%20First%20Person%20Char)) (.StaticMeshTemp-Delete-AfterAddingToolMechanic (Utilities|Struct|BreakSInspectableObjectData _returnvalue)))))))