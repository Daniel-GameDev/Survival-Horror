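; Tunnel elevator actor that rides along a spline path, starting automatically at BeginPlay.
; It finds the BP_TunnelSplinePath actor in the level, then plays a timeline with its rate scaled by TimeToComplete.
; Each update lerps distance between the first two spline points and sets its world location there, without sweeping or changing rotation.
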(event Custom|MoveElevator
  (Components|Timeline|SetPlayRate (Variables|Default|GetMoveElevatorTime) (/ 1.0 (Variables|Default|GetTimeToComplete)))
  (bind _movetrack (Timeline|MoveElevatorTime Play)
    (:Update
      (Transformation|SetActorLocation (Spline|GetLocationatDistanceAlongSpline (Variables|/Game/SurvivalHorror/Maps/Parallel/Assets/Blueprints/Tunnel/BP_TunnelSplinePath.BP_TunnelSplinePath_C|GetSpline (Variables|Default|GetSpline_Ref)) (Math|Float|Lerp (Spline|GetDistanceAlongSplineatSplinePoint (Variables|/Game/SurvivalHorror/Maps/Parallel/Assets/Blueprints/Tunnel/BP_TunnelSplinePath.BP_TunnelSplinePath_C|GetSpline (Variables|Default|GetSpline_Ref)) 0) (Spline|GetDistanceAlongSplineatSplinePoint (Variables|/Game/SurvivalHorror/Maps/Parallel/Assets/Blueprints/Tunnel/BP_TunnelSplinePath.BP_TunnelSplinePath_C|GetSpline (Variables|Default|GetSpline_Ref)) 1) _movetrack) "World") false false))))

(event EventBeginPlay
  (bind _returnvalue (Actor|GetActorOfClass "/Game/SurvivalHorror/Maps/Parallel/Assets/Blueprints/Tunnel/BP_TunnelSplinePath.BP_TunnelSplinePath_C"))
  (Variables|Default|SetSpline_Ref _returnvalue)
  (CallFunction|MoveElevator))

(fn ConstructionScript)