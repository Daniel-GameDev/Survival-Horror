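; BP_Container is an interactable container actor that opens its contents for the interacting pawn through an ACContainer component.
; Interact fires the Interacting event, which clears TakesTimeToInteract through a DoOnce, removing the interaction delay after first use, then calls OpenContainer.
; GetContent exposes the component's Content array, and DeleteItem overwrites the given slot with an empty value rather than removing it.
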(event Custom|DisableDelayInteraction
  (Utilities|FlowControl|DoOnce false
    (:Completed
      (Variables|Default|SetTakesTimeToInteract false))))

(event EventBeginPlay
  (|CallParentFunction) ; This node is disabled and will not be called.\nDrag off pins to build functionality.
)

(event Collision|EventActorBeginOverlap
  (params (OtherActor :type Actor%20Object%20Reference)))

(event EventTick
  (params (DeltaSeconds :type Float%20%28single-precision%29))
  (|CallParentFunction DeltaSeconds) ; This node is disabled and will not be called.\nDrag off pins to build functionality.
)

(event EventInteracting
  (params (Interacter :type Pawn%20Object%20Reference))
  (Utilities|FlowControl|Sequence
    (:then_0
      (Utilities|FlowControl|DoOnce false
        (:Completed
          (Variables|Default|SetTakesTimeToInteract false))))
    (:then_1
      (Default|OpenContainer (Variables|Default|GetAC_Container) Interacter))))

(fn ConstructionScript
  (|CallParentFunction))

(fn Interact
  (params (Interacter :type Primitive%20Component%20Object%20Reference) (Pawn :type BP%20First%20Person%20Char%20Object%20Reference))
  (CallFunction|Interacting Pawn)
  (return true "NewEnumerator5"))

(fn DeleteItem
  (params (Index :type Integer))
  (Utilities|Array|SetArrayElem :TargetArray (Variables|/Game/SurvivalHorror/Assets/GameplayActors/GymElements/Gym_Inventory/CustomInventory/AC_Inventory.AC_Inventory_C|GetContent (Variables|Default|GetAC_Container)) :Index Index))

(fn GetContent
  (return (Variables|/Game/SurvivalHorror/Assets/GameplayActors/GymElements/Gym_Inventory/CustomInventory/AC_Inventory.AC_Inventory_C|GetContent (Variables|Default|GetAC_Container))))