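; Base actor for inspectable items that the first-person player examines up close, loading item data from DT_ItemData by ItemId at construction.
; Interacting hands input to the item, attaches it to the character's view-point arrow, raises it by timeline, then shows post-process and WBP_InspectableScreen.
; Look axes rotate the mesh.
; LMB stores eligible types in AC_Inventory and destroys the actor, RMB returns it to its saved transform, and Drop releases it with physics.
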(event Custom|DropFrom
  (Physics|SetSimulatePhysics (Variables|Default|GetStaticMesh) true)
  (Collision|SetCollisionResponsetoChannel (Variables|Default|GetStaticMesh) "ECC_Pawn" "ECR_Ignore")
  (Collision|SetCollisionEnabled (Variables|Default|GetStaticMesh) "QueryAndPhysics"))

(event EventBeginPlay
  (|CallParentFunction) ; This node is disabled and will not be called.\nDrag off pins to build functionality.
)

(event Collision|EventActorBeginOverlap
  (params (OtherActor :type Actor%20Object%20Reference)))

(event EventTick
  (params (DeltaSeconds :type Float%20%28single-precision%29))
  (|CallParentFunction DeltaSeconds) ; This node is disabled and will not be called.\nDrag off pins to build functionality.
)

(event EventInteracting
  (params (Interacter :type Pawn%20Object%20Reference))
  (bind _inspectableobjectdata (Variables|Default|GetInspectableObjectData))
  (Input|DisableInput Interacter (Game|GetPlayerController 0))
  (if (Physics|IsSimulatingPhysics (Variables|Default|GetStaticMesh) "None")
    (Physics|SetSimulatePhysics (Variables|Default|GetStaticMesh) false))
  (bind _asbp_first_person_char (Utilities|Casting|CastToBP_FirstPerson_Char Interacter))
  (Variables|Default|SetPickupTransform (Transformation|GetWorldTransform (Variables|Default|GetStaticMesh)))
  (Variables|Default|SetRelative%20Rotation (Variables|/Script/Engine.SceneComponent|GetRelativeRotation (Variables|Default|GetStaticMesh)))
  (Variables|Default|SetAs%20BP%20First%20Person%20Char _asbp_first_person_char)
  (Variables|Default|SetFirst%20Person%20Camera (Variables|/Game/SurvivalHorror/Assets/Characters/FirstPerson/Main/BP_FirstPerson_Char.BP_FirstPerson_Char_C|GetFirstPersonCamera _asbp_first_person_char))
  (Variables|Default|SetMy%20Inspectable%20Arrow%20End (Variables|/Game/SurvivalHorror/Assets/Characters/FirstPerson/Main/BP_FirstPerson_Char.BP_FirstPerson_Char_C|GetMyInspectableArrowEnd _asbp_first_person_char))
  (Variables|Default|SetMy%20Inspectable%20Arrow%20View%20Point (Variables|/Game/SurvivalHorror/Assets/Characters/FirstPerson/Main/BP_FirstPerson_Char.BP_FirstPerson_Char_C|GetMyInspectableArrowViewPoint _asbp_first_person_char))
  (Variables|Default|SetMy%20Inspectable%20Arrow%20Start (Variables|/Game/SurvivalHorror/Assets/Characters/FirstPerson/Main/BP_FirstPerson_Char.BP_FirstPerson_Char_C|GetMyInspectableArrowStart _asbp_first_person_char))
  (Input|EnableInput (Game|GetPlayerController 0))
  (Collision|SetCollisionEnabled (Variables|Default|GetStaticMesh) "NoCollision")
  (Transformation|AttachComponentToComponent (Variables|Default|GetMy%20Inspectable%20Arrow%20View%20Point) "None" "SnapToTarget" "SnapToTarget" "KeepWorld" false)
  (bind _swap (Timeline|ItemSwapVie PlayFromStart)
    (:Update
      (Transformation|SetRelativeLocation (Variables|Default|GetMy%20Inspectable%20Arrow%20View%20Point) (Math|Vector|MakeVector (.x (Variables|/Script/Engine.SceneComponent|GetRelativeLocation (Variables|Default|GetMy%20Inspectable%20Arrow%20Start))) (.y (Variables|/Script/Engine.SceneComponent|GetRelativeLocation (Variables|Default|GetMy%20Inspectable%20Arrow%20Start))) (Math|Float|Lerp (.z (Variables|/Script/Engine.SceneComponent|GetRelativeLocation (Variables|Default|GetMy%20Inspectable%20Arrow%20Start))) (.z (Variables|/Script/Engine.SceneComponent|GetRelativeLocation (Variables|Default|GetMy%20Inspectable%20Arrow%20End))) _swap)) false false))
    (:Finished
      (Variables|Default|SetPost%20Process%20Save (Variables|/Script/Engine.CameraComponent|GetPostProcessSettings (Variables|Default|GetFirst%20Person%20Camera)))
      (Variables|/Script/Engine.CameraComponent|SetPostProcessSettings (Variables|Default|GetFirst%20Person%20Camera) (Variables|Default|GetPost%20Process%20Settings))
      (Class|CameraComponent|SetPostProcessBlendWeight (Variables|Default|GetFirst%20Person%20Camera) 1.0)
      (bind _returnvalue (UserInterface|CreateWidget "/Game/SurvivalHorror/Assets/GameplayActors/GymElements/Common/Widgets/WBP_InspectableScreen.WBP_InspectableScreen_C" (Game|GetPlayerController 0) (.name _inspectableobjectdata) (.description _inspectableobjectdata) (.icon _inspectableobjectdata) (.type _inspectableobjectdata)))
      (bind _output_get (Variables|Default|SetInspectWidget _returnvalue))
      (UserInterface|Viewport|AddtoViewport _output_get 0))))

(event Input|ActionEvents|InputActionLMBAction
  (params (Key :type Key%20Structure :default "None"))
  (bind _my_inspectable_arrow_view_point (Variables|Default|GetMy%20Inspectable%20Arrow%20View%20Point))
  (bind _as_bp_first_person_char (Variables|Default|GetAs%20BP%20First%20Person%20Char))
  (bind _returnvalue (Actor|GetComponentbyClass _as_bp_first_person_char "/Game/SurvivalHorror/Assets/GameplayActors/GymElements/Gym_Inventory/CustomInventory/AC_Inventory.AC_Inventory_C"))
  (bind _relativelocation (Variables|/Script/Engine.SceneComponent|GetRelativeLocation _my_inspectable_arrow_view_point))
  (:Pressed
    (if (Utilities|Enum|NotEqual(Enum) (.type (Variables|Default|GetInspectableObjectData)) "NewEnumerator0")
      (Utilities|IsValid _returnvalue
        (:Is%20Valid
          (bind _hasemptyslot (Default|AddItem _returnvalue (Variables|Default|GetItemId)))
          (if _hasemptyslot
            (Input|DisableInput (Game|GetPlayerController 0))
            (Transformation|DetachFromActor "KeepWorld" "KeepWorld" "KeepWorld")
            (Input|EnableInput (Variables|Default|GetAs%20BP%20First%20Person%20Char) (Game|GetPlayerController 0))
            (Class|CameraComponent|SetPostProcessBlendWeight (Variables|Default|GetFirst%20Person%20Camera) 0.0)
            (Default|BreakInteraction (Variables|Default|GetAs%20BP%20First%20Person%20Char))
            (bind _inspectwidget (Variables|Default|GetInspectWidget)
              (:then
                (Widget|RemovefromParent _inspectwidget))
              (:else
                _))
            (Transformation|SetRelativeLocation (Variables|Default|GetMy%20Inspectable%20Arrow%20View%20Point) (Math|Vector|MakeVector (.x _relativelocation) (.y _relativelocation) (.z (Variables|/Script/Engine.SceneComponent|GetRelativeLocation (Variables|Default|GetMy%20Inspectable%20Arrow%20Start)))) false true)
            (Actor|DestroyActor)))))))

(event Input|ActionEvents|InputActionRMBAction
  (params (Key :type Key%20Structure :default "None"))
  (bind _my_inspectable_arrow_view_point (Variables|Default|GetMy%20Inspectable%20Arrow%20View%20Point))
  (bind _relativelocation (Variables|/Script/Engine.SceneComponent|GetRelativeLocation _my_inspectable_arrow_view_point))
  (:Pressed
    (Input|DisableInput (Game|GetPlayerController 0))
    (bind _swap (Timeline|Timeline_0 ReverseFromEnd)
      (:Update
        (Transformation|SetRelativeLocation (Variables|Default|GetMy%20Inspectable%20Arrow%20View%20Point) (Math|Vector|MakeVector (.x _relativelocation) (.y _relativelocation) (Math|Float|Lerp (.z (Variables|/Script/Engine.SceneComponent|GetRelativeLocation (Variables|Default|GetMy%20Inspectable%20Arrow%20Start))) (.z (Variables|/Script/Engine.SceneComponent|GetRelativeLocation (Variables|Default|GetMy%20Inspectable%20Arrow%20End))) _swap)) false false))
      (:Finished
        (Transformation|SetRelativeRotation (Variables|Default|GetStaticMesh) (Variables|Default|GetRelative%20Rotation) false false)
        (Transformation|DetachFromActor "KeepWorld" "KeepWorld" "KeepWorld")
        (Transformation|SetWorldTransform (Variables|Default|GetStaticMesh) (Variables|Default|GetPickupTransform) false true)
        (Input|EnableInput (Variables|Default|GetAs%20BP%20First%20Person%20Char) (Game|GetPlayerController 0))
        (Collision|SetCollisionEnabled (Variables|Default|GetStaticMesh) "QueryAndPhysics")
        (Class|CameraComponent|SetPostProcessBlendWeight (Variables|Default|GetFirst%20Person%20Camera) 0.0)
        (Default|BreakInteraction (Variables|Default|GetAs%20BP%20First%20Person%20Char))
        (Widget|RemovefromParent (Variables|Default|GetInspectWidget))))))

(event Input|ActionEvents|InputActionDrop
  (params (Key :type Key%20Structure :default "None"))
  (bind _my_inspectable_arrow_view_point (Variables|Default|GetMy%20Inspectable%20Arrow%20View%20Point))
  (bind _relativelocation (Variables|/Script/Engine.SceneComponent|GetRelativeLocation _my_inspectable_arrow_view_point))
  (:Pressed
    (Input|DisableInput (Game|GetPlayerController 0))
    (Transformation|SetRelativeRotation (Variables|Default|GetStaticMesh) (Variables|Default|GetRelative%20Rotation) false false)
    (Transformation|DetachFromActor "KeepWorld" "KeepWorld" "KeepWorld")
    (Physics|SetSimulatePhysics (Variables|Default|GetStaticMesh) true)
    (Collision|SetCollisionResponsetoChannel (Variables|Default|GetStaticMesh) "ECC_Pawn" "ECR_Ignore")
    (Input|EnableInput (Variables|Default|GetAs%20BP%20First%20Person%20Char) (Game|GetPlayerController 0))
    (Collision|SetCollisionEnabled (Variables|Default|GetStaticMesh) "QueryAndPhysics")
    (Class|CameraComponent|SetPostProcessBlendWeight (Variables|Default|GetFirst%20Person%20Camera) 0.0)
    (Default|BreakInteraction (Variables|Default|GetAs%20BP%20First%20Person%20Char))
    (Widget|RemovefromParent (Variables|Default|GetInspectWidget))
    (Transformation|SetRelativeLocation (Variables|Default|GetMy%20Inspectable%20Arrow%20View%20Point) (Math|Vector|MakeVector (.x _relativelocation) (.y _relativelocation) (.z (Variables|/Script/Engine.SceneComponent|GetRelativeLocation (Variables|Default|GetMy%20Inspectable%20Arrow%20Start)))) false true)))

(event Input|AxisEvents|InputAxisTurn
  (params (AxisValue :type Float%20%28single-precision%29))
  (bind _staticmesh (Variables|Default|GetStaticMesh))
  (Transformation|SetRelativeRotation _staticmesh (Math|Rotator|CombineRotators (Variables|/Script/Engine.SceneComponent|GetRelativeRotation _staticmesh) (Math|Rotator|MakeRotator 0.0 0.0 (/ AxisValue 2.0))) false false))

(event Input|AxisEvents|InputAxisLookUp
  (params (AxisValue :type Float%20%28single-precision%29))
  (bind _staticmesh (Variables|Default|GetStaticMesh))
  (Transformation|SetRelativeRotation _staticmesh (Math|Rotator|CombineRotators (Variables|/Script/Engine.SceneComponent|GetRelativeRotation _staticmesh) (Math|Rotator|MakeRotator 0.0 (/ AxisValue 2.0) 0.0)) false false))

(fn ConstructionScript
  (|CallParentFunction)
  (bind _returnvalue (Utilities|GetDataTableRow "/Game/SurvivalHorror/Assets/GameplayActors/GymElements/Gym_Inventory/CustomInventory/DT_ItemData.DT_ItemData" (Variables|Default|GetItemId))
    (:then
      (Variables|Default|SetInspectableObjectData (Utilities|Struct|MakeSInspectableObjectData (.name _returnvalue) (.description _returnvalue) (.icon _returnvalue) (.type _returnvalue) (.class _returnvalue) (.stacksize _returnvalue) (.staticmeshtemp-delete-afteraddingtoolmechanic _returnvalue))))))

(fn Interact
  (params (Interacter :type Primitive%20Component%20Object%20Reference) (Pawn :type BP%20First%20Person%20Char%20Object%20Reference))
  (CallFunction|Interacting Pawn)
  (return true "NewEnumerator4"))