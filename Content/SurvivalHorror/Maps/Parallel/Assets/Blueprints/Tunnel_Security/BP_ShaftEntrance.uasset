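; BP_ShaftEntrance is an interactable shaft entrance that opens when the player uses it while carrying a screwdriver.
; On interaction it casts to the first-person character and searches its inventory component for the Screwdriver item, then destroys the door component once.
; A disconnected node would spawn a heavy-object shaft door at the door's relative transform, but it never runs.
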(event EventInteracting
  (params (Interacter :type Pawn%20Object%20Reference))
  (bind _asbp_first_person_char (Utilities|Casting|CastToBP_FirstPerson_Char Interacter))
  (for _array_element (Variables|/Game/SurvivalHorror/Assets/GameplayActors/GymElements/Gym_Inventory/CustomInventory/AC_Inventory.AC_Inventory_C|GetContent (Variables|/Game/SurvivalHorror/Assets/Characters/FirstPerson/Main/BP_FirstPerson_Char.BP_FirstPerson_Char_C|GetAC_Inventory _asbp_first_person_char))
    (if (Utilities|Name|Equal(Name) (.itemid _array_element) "Screwdriver")
      (Utilities|FlowControl|DoOnce false
        (:Completed
          (Components|DestroyComponent (Variables|Default|GetShaftDoor)))))))

(fn ConstructionScript)