(event Custom|CameraFadeOut3
  (bind _outactors (Actor|GetAllActorsOfClass "/Script/Engine.StaticMeshActor"))
  (bind _array_element (Utilities|Array|ForEachLoopwithBreak _outactors)
    (:LoopBody
      (if (Utilities|Enum|Equal(Enum) (Utilities|GetObjectName _array_element) "Floor_3")
        (Rendering|Material|SetMaterial (Variables|/Script/Engine.StaticMeshActor|GetStaticMeshComponent _array_element) 0 "/Game/SurvivalHorror/Assets/MasterMaterials/Water/Materials/M_Water_Red.M_Water_Red")
        (CameraFades|StartCameraFade :self (Game|GetPlayerCameraManager 0) :FromAlpha 1.0 :Duration 5.0)))))

(event Custom|CameraFadeOut1
  (CameraFades|StartCameraFade (Game|GetPlayerCameraManager 0) 0.5 0.0 4.0 "(R=0.052083,G=0.001320,B=0.000000,A=1.000000)" false false))

(event Custom|CameraFadeout2
  (Utilities|FlowControl|Sequence
    (:then_0
      (bind _outactors (Actor|GetAllActorsOfClass "/Script/Engine.AtmosphericFog"))
      (bind _array_element (Utilities|Array|ForEachLoopwithBreak _outactors)
        (:LoopBody
          (Class|AtmosphericFogComponent|SetDefaultLightColor (Variables|/Script/Engine.AtmosphericFog|GetAtmosphericFogComponent _array_element) "(R=0.338542,G=0.000000,B=0.000000,A=1.000000)"))))
    (:then_1
      (bind _outactors_2 (Actor|GetAllActorsOfClass "/Script/Engine.DirectionalLight"))
      (bind _array_element_2 (Utilities|Array|ForEachLoopwithBreak _outactors_2)
        (:LoopBody
          (Rendering|Components|Light|SetLightColor (Variables|/Script/Engine.Light|GetLightComponent _array_element_2) "(R=1.000000,G=0.000000,B=0.000000,A=1.000000)" true)
          (CameraFades|StartCameraFade :self (Game|GetPlayerCameraManager 0) :FromAlpha 1.0 :Duration 5.0))))))

(event Custom|CameraFade4
  (Game|Damage|ApplyDamage (Variables|Default|GetOtherActor) 1e+02 0 self)
  (CameraFades|StartCameraFade (Game|GetPlayerCameraManager 0) 1.0 0.2 5.0 "(R=0.024158,G=0.000000,B=0.001214,A=1.000000)" false true))

(event EventStartMentalAnomaly
  (params (Value :type Float%20%28single-precision%29))
  (if (== Value 3.0)
    (Audio|PlaySound2D "/Game/SurvivalHorror/Assets/GameplayActors/GymElements/Mental/Sounds/A_Whispers1.A_Whispers1" 0.05 0.8 0.0 0 0 false)
    (CameraFades|StartCameraFade (Game|GetPlayerCameraManager 0) 0.0 0.5 4.0 "(R=0.052083,G=0.001320,B=0.000000,A=1.000000)" false false)
    (Utilities|Time|SetTimerbyEvent (delegate Custom|CameraFadeOut1) 4.0)
    (elif (== Value 2.0)
      (Audio|PlaySound2D "/Game/SurvivalHorror/Assets/GameplayActors/GymElements/Mental/Sounds/A_BackgroundCaveWhispers.A_BackgroundCaveWhispers" 0.1 0.7 0.0 0 0 false)
      (CameraFades|StartCameraFade :self (Game|GetPlayerCameraManager 0) :ToAlpha 1.0 :Duration 3.0 :bHoldWhenFinished true)
      (Utilities|Time|SetTimerbyEvent (delegate Custom|CameraFadeout2) 4.0)
      (elif (== Value 1.0)
        (Audio|PlaySound2D "/Game/SurvivalHorror/Assets/GameplayActors/GymElements/Mental/Sounds/A_LongWhispers.A_LongWhispers" 0.1 0.7 0.0 0 0 false)
        (CameraFades|StartCameraFade :self (Game|GetPlayerCameraManager 0) :ToAlpha 1.0 :Duration 3.0 :bHoldWhenFinished true)
        (Utilities|Time|SetTimerbyEvent (delegate Custom|CameraFadeOut3) 4.0)
        (elif (== Value 0.0)
          (Audio|PlaySound2D "/Game/SurvivalHorror/Assets/GameplayActors/GymElements/Mental/Sounds/A_WhispersHit.A_WhispersHit" 5.0 0.7 0.0 0 0 false)
          (CameraFades|StartCameraFade (Game|GetPlayerCameraManager 0) 0.0 1.0 2.5 "(R=0.025187,G=0.000000,B=0.001214,A=1.000000)" false true)
          (Utilities|Time|SetTimerbyEvent (delegate Custom|CameraFade4) 3.0))))))

(event Collision|EventActorBeginOverlap
  (params (OtherActor :type Actor%20Object%20Reference))
  (Variables|Default|SetOtherActor OtherActor))

(event Collision|EventActorEndOverlap
  (params (OtherActor :type Actor%20Object%20Reference))
  (Variables|Default|SetOtherActor 0))

(fn ConstructionScript)