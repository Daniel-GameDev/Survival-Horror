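; BP_TunnelGates_Large is a large two-door tunnel gate that slides open or closed through its OpenGates event.
; A timeline, with play rate set from TimeToComplete on BeginPlay, lerps the left and right doors apart along relative X.
; Open plays it and Close reverses it, gated by a GatesOpened flag that toggles when the timeline finishes.
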(event Custom|OpenGates
  (params (GatesAction :type EGatesAction%20Enum :default "NewEnumerator0"))
  (bind _gatesdoorleft (Variables|Default|GetGatesDoorLeft))
  (bind _gatesdoorright (Variables|Default|GetGatesDoorRight))
  (bind _relativelocation (Variables|/Script/Engine.SceneComponent|GetRelativeLocation _gatesdoorleft))
  (bind _relativelocation_2 (Variables|/Script/Engine.SceneComponent|GetRelativeLocation _gatesdoorright))
  (switch Utilities|FlowControl|Switch|SwitchonEGatesAction GatesAction
    (:NewEnumerator0
      (if (not (Variables|Default|GetGatesOpened))
        (bind _openning (Timeline|OpenGatesTimeLine Play)
          (:Update
            (Transformation|SetRelativeLocation _gatesdoorleft (Math|Vector|MakeVector (Math|Float|Lerp -1e+02 5e+02 _openning) (.y _relativelocation) (.z _relativelocation)) false false)
            (Transformation|SetRelativeLocation _gatesdoorright (Math|Vector|MakeVector (Math|Float|Lerp 1e+02 -5e+02 _openning) (.y _relativelocation_2) (.z _relativelocation_2)) false false))
          (:Finished
            (if (Variables|Default|GetGatesOpened)
              (Variables|Default|SetGatesOpened false)
              (else
                (Variables|Default|SetGatesOpened true)))))))
    (:NewEnumerator1
      (if (Variables|Default|GetGatesOpened)
        (Timeline|OpenGatesTimeLine Reverse)))))

(event EventBeginPlay
  (Components|Timeline|SetPlayRate (Variables|Default|GetOpenGatesTimeLine) (/ 1.0 (Variables|Default|GetTimeToComplete))))

(fn ConstructionScript)