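; Inventory actor component for a first-person character, storing item stacks in a fixed-size slot array.
; Adding fills matching stacks up to DataTable limits, then empty slots; removal is an empty stub.
; A per-tick camera sphere trace prints look-at messages, while a server RPC triggers item interaction.
; Slot transfers handle differing items, writing both swapped entries into the source inventory, then multicast updates on both components.
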(event Custom|Server_Interact
  (params (Target :type Actor%20Object%20Reference))
  (bind _returnvalue (Actor|GetComponentbyClass Target "/Game/SurvivalHorror/Assets/GameplayActors/GymElements/Gym_Inventory/BPC_ItemData_InvT1.BPC_ItemData_InvT1_C"))
  ;[1 0 0] Replicated Event > Replicates > RunOnServer
  (Utilities|IsValid _returnvalue
    (:Is%20Valid
      (Class|BPIInteractInterfaceInvT1|Interactwith(Message) _returnvalue (.AsBP%20First%20Person%20Char (Utilities|Casting|CastToBP_FirstPerson_Char (Components|GetOwner)))))))

(event Custom|CallDebug
  (CallFunction|DEBUGPrintContents))

(event Custom|MC_Update
  ;[1 0 0] MultiCastUpdate Replicates > Multicast
  (Default|CallOnInventoryUpdated))

(event Custom|SERVER_TransferSlots
  (params (SourceIndex :type Integer) (SourceInventory :type BPC%20Inventory%20System%20Inv%20T1%20Object%20Reference) (DestinationIndex :type Integer))
  (CallFunction|TransferSlots SourceIndex SourceInventory DestinationIndex))

(event EventBeginPlay
  (Utilities|Array|Resize (Variables|Default|GetContent) (Variables|Default|GetInventorySize)))

(event EventTick
  (params (DeltaSeconds :type Float%20%28single-precision%29))
  (CallFunction|InteractionTrace))

(fn AddtoInventory
  (params (ItemID :type Name) (Quantity :type Integer))
  (LocalVariables|SetLocal_QuantityRemaining Quantity)
  (while (Math|Boolean|Equal(Boolean) (> (LocalVariables|GetLocal_QuantityRemaining) 0) (not (LocalVariables|GetLocal_HasFailed)))
    (bind (_index _foundslot) (CallFunction|FindSlot ItemID))
    (if _foundslot
      (CallFunction|AddtoStack _index 1)
      (Math|Integer|DecrementInt (LocalVariables|GetLocal_QuantityRemaining))
      (elif (.HasEmptySlot (CallFunction|AnyEmptySlotsAvailable))
        (bind _success (CallFunction|CreateNewStack ItemID 1))
        (if _success
          (Math|Integer|DecrementInt (LocalVariables|GetLocal_QuantityRemaining))
          (else
            (LocalVariables|SetLocal_HasFailed true)))
        (else
          (LocalVariables|SetLocal_HasFailed true)))))
  (return (not (LocalVariables|GetLocal_HasFailed)) (LocalVariables|GetLocal_QuantityRemaining)))

(fn RemovefromInventory)

(fn InteractionTrace
  (bind _returnvalue (Game|GetPlayerCameraManager 0))
  (bind _returnvalue_2 (Transformation|GetActorLocation _returnvalue))
  (bind (_outhit _returnvalue_3) (Collision|SphereTraceByChannel _returnvalue_2 (+ _returnvalue_2 (* (Transformation|GetActorForwardVector _returnvalue) (Variables|Default|GetInteractionRange))) 15.0 "TraceTypeQuery3" true (Utilities|Array|MakeArray (Components|GetOwner)) "ForOneFrame"))
  (if _returnvalue_3
    (if (!= (.HitActor (Collision|BreakHitResult _outhit)) (Variables|Default|GetLookAtActor))
      (bind _output_get (Variables|Default|SetLookAtActor (.HitActor (Collision|BreakHitResult _outhit))))
      (bind _message (Class|BPIInteractInterfaceInvT1|Lookat(Message) _output_get))
      (Development|PrintString (Utilities|String|ToString(Text) _message)))
    (else
      (Variables|Default|SetLookAtActor 0))))

(fn FindSlot
  (params (ItemID :type Name))
  (for (_array_element _array_index) (Variables|Default|GetContent)
    (if (Utilities|Name|Equal(Name) (.ItemID (Utilities|Struct|BreakFSlotStruct_InvT1 _array_element)) ItemID)
      (if (< (.Quantity (Utilities|Struct|BreakFSlotStruct_InvT1 _array_element)) (CallFunction|GetMaxStackSize ItemID))
        (return _array_index true))))
  ;[1 0 0] Negative Value means NoValue
  (return -1 false))

(fn GetMaxStackSize
  (params (ItemID :type Name))
  (bind _returnvalue (Utilities|GetDataTableRow "/Game/SurvivalHorror/Assets/GameplayActors/GymElements/Gym_Inventory/DT_ItemData_InvT1.DT_ItemData_InvT1" ItemID)
    (:then
      (return (.stacksize _returnvalue)))
    (:RowNotFound
      ;[1 0 0] Negative Value means NoValue
      (return -1))))

(fn AddtoStack
  (params (Index :type Integer) (Quantity :type Integer))
  (bind _content (Variables|Default|GetContent))
  (bind _output (Utilities|Array|Get(acopy) _content Index))
  (Utilities|Array|SetArrayElem (Variables|Default|GetContent) Index (Utilities|Struct|MakeFSlotStruct_InvT1 (.itemid _output) (+ (.quantity _output) Quantity))))

(fn AnyEmptySlotsAvailable
  (for (_array_element _array_index) (Variables|Default|GetContent)
    (if (== (.Quantity (Utilities|Struct|BreakFSlotStruct_InvT1 _array_element)) 0)
      (return _array_index true)))
  (return -1 false))

(fn CreateNewStack
  (params (ItemID :type Name) (Quantity :type Integer))
  (bind (_index _hasemptyslot) (CallFunction|AnyEmptySlotsAvailable))
  (if _hasemptyslot
    (Utilities|Array|SetArrayElem (Variables|Default|GetContent) _index (Utilities|Struct|MakeFSlotStruct_InvT1 ItemID Quantity))
    (return true)
    (else
      (return false))))

(fn DEBUGPrintContents
  (for (_array_element _array_index) (Variables|Default|GetContent)
    (Development|PrintString (Utilities|String|Append (Utilities|String|ToString(Integer) _array_index) " " (Utilities|String|ToString(Name) (.ItemID (Utilities|Struct|BreakFSlotStruct_InvT1 _array_element))) " = " (Utilities|String|ToString(Integer) (.Quantity (Utilities|Struct|BreakFSlotStruct_InvT1 _array_element)))))))

(fn TransferSlots
  (params (SourceIndex :type Integer) (SourceInventory :type BPC%20Inventory%20System%20Inv%20T1%20Object%20Reference) (DestinationIndex :type Integer))
  (LocalVariables|SetLocal_SlotContent (Utilities|Array|Get(acopy) (Variables|BPC_InventorySystem_InvT1_C|GetContent SourceInventory) SourceIndex))
  (if (not (< DestinationIndex 0))
    (if (not (Utilities|Name|Equal(Name) (.ItemID (Utilities|Struct|BreakFSlotStruct_InvT1 (LocalVariables|GetLocal_SlotContent))) (.ItemID (Utilities|Struct|BreakFSlotStruct_InvT1 (Utilities|Array|Get(acopy) (Variables|Default|GetContent) DestinationIndex)))))
      (Utilities|Array|SetArrayElem (Variables|BPC_InventorySystem_InvT1_C|GetContent SourceInventory) SourceIndex (Utilities|Array|Get(acopy) (Variables|Default|GetContent) DestinationIndex))
      (Utilities|Array|SetArrayElem (Variables|BPC_InventorySystem_InvT1_C|GetContent SourceInventory) DestinationIndex (LocalVariables|GetLocal_SlotContent))
      (CallFunction|MCUpdate)
      (CallFunction|MCUpdate SourceInventory))))