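; Parent Blueprint for pushable physics objects, supplying a default "Push" prompt and focus icons unless custom settings are enabled.
; When a first-person interface actor overlaps the Box, the mesh's physics is disabled while that actor reports an interacting message.
; A 0.2-second timer re-checks this state, restoring physics once interaction or overlap ends and optionally hiding the inner billboard.
; Interact only returns the permanent-use flag and object type.
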(event OnComponentBeginOverlap(Box)
  (params (OverlappedComponent :type Primitive%20Component%20Object%20Reference) (OtherActor :type Actor%20Object%20Reference) (OtherComp :type Primitive%20Component%20Object%20Reference) (OtherBodyIndex :type Integer) (bFromSweep :type Boolean) (SweepResult :type Hit%20Result%20Structure%20%28by%20ref%29))
  (bind _returnvalue (Components|GetOwner OtherComp))
  (if (Utilities|DoesObjectImplementInterface _returnvalue "/Game/SurvivalHorror/Assets/Characters/FirstPerson/Main/BPI_FirstPerson.BPI_FirstPerson_C")
    (bind _output_get (Variables|Default|SetOther%20Comp OtherComp))
    (bind _busy (Class|BPIFirstPerson|GetInteracting(Message) _returnvalue))
    (if _busy
      (Physics|SetSimulatePhysics (Variables|Default|GetStaticMesh) false)
      (bind _returnvalue_2 (Utilities|Time|SetTimerbyEvent (delegate Custom|RecallInteracting) 0.2))
      (else
        (Utilities|Time|ClearandInvalidateTimerbyHandle _returnvalue_2)
        (Physics|SetSimulatePhysics (Variables|Default|GetStaticMesh) true)
        (if (Variables|PushableSettings|GetHideBillboardsOnTouch)
          (Default|SetBillboardVisibility self true false))))))

(event OnComponentEndOverlap(Box)
  (params (OverlappedComponent :type Primitive%20Component%20Object%20Reference) (OtherActor :type Actor%20Object%20Reference) (OtherComp :type Primitive%20Component%20Object%20Reference) (OtherBodyIndex :type Integer)))

(event Custom|RecallInteracting
  (if (Utilities|Array|ContainsItem (Class|PrimitiveComponent|GetOverlappingComponents (Variables|Default|GetBox)) (stale OnComponentBeginOverlap(Box) _output_get))
    (bind _busy (Class|BPIFirstPerson|GetInteracting(Message) (Components|GetOwner (stale OnComponentBeginOverlap(Box) OtherComp))))
    (if _busy
      (Physics|SetSimulatePhysics (Variables|Default|GetStaticMesh) false)
      (bind _returnvalue (Utilities|Time|SetTimerbyEvent (delegate Custom|RecallInteracting) 0.2))
      (else
        (Utilities|Time|ClearandInvalidateTimerbyHandle _returnvalue :!label _label)
        (Physics|SetSimulatePhysics (Variables|Default|GetStaticMesh) true)
        (if (Variables|PushableSettings|GetHideBillboardsOnTouch)
          (Default|SetBillboardVisibility self true false))))
    (else
      (goto _label))))

(event EventBeginPlay
  (bind _self self)
  ;[1 0 0] Check out Class Defaults
  (if (Variables|PushableSettings|GetUseCustomSettings)
    (|CallParentFunction :!label _label)
    (else
      (Utilities|FlowControl|Sequence
        (:then_0
          (Variables|/Game/SurvivalHorror/Assets/GameplayActors/GymElements/Common/BP_InteractableObject_Parent.BP_InteractableObject_Parent_C|SetStencilValue _self 0))
        (:then_1
          (Variables|/Game/SurvivalHorror/Assets/GameplayActors/GymElements/Common/BP_InteractableObject_Parent.BP_InteractableObject_Parent_C|SetDrawDotOnFocus _self false))
        (:then_2
          (Variables|/Game/SurvivalHorror/Assets/GameplayActors/GymElements/Common/BP_InteractableObject_Parent.BP_InteractableObject_Parent_C|SetInnerIcon _self "NewEnumerator0"))
        (:then_3
          (Variables|/Game/SurvivalHorror/Assets/GameplayActors/GymElements/Common/BP_InteractableObject_Parent.BP_InteractableObject_Parent_C|SetOuterIcon _self "NewEnumerator0"))
        (:then_4
          (Variables|/Game/SurvivalHorror/Assets/GameplayActors/GymElements/Common/BP_InteractableObject_Parent.BP_InteractableObject_Parent_C|SetPermanent%20Using _self false))
        (:then_5
          (Variables|/Game/SurvivalHorror/Assets/GameplayActors/GymElements/Common/BP_InteractableObject_Parent.BP_InteractableObject_Parent_C|SetMessage _self "Push"))
        (:then_6
          (goto _label))))))

(event Collision|EventActorBeginOverlap
  (params (OtherActor :type Actor%20Object%20Reference))
  (|CallParentFunction OtherActor) ; This node is disabled and will not be called.\nDrag off pins to build functionality.
)

(event EventTick
  (params (DeltaSeconds :type Float%20%28single-precision%29))
  ;[1 0 0] Check out Class Defaults
  (|CallParentFunction DeltaSeconds) ; This node is disabled and will not be called.\nDrag off pins to build functionality.
)

(fn ConstructionScript
  (|CallParentFunction))

(fn Interact
  (params (Interacter :type Primitive%20Component%20Object%20Reference))
  (return (Variables|Default|GetPermanent%20Using self) "NewEnumerator0"))