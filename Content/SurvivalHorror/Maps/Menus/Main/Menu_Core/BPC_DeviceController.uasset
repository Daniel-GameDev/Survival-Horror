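; BPC_DeviceController is a menu component that tracks whether the player is using keyboard/mouse or gamepad.
; SwitchCurrentDevice classifies the supplied key and calls SwitchInputDevice only when the device type changes.
; OnMouseMovement switches from gamepad back to mouse when the cursor differs from the default-resolution coordinates, printing a debug string.
; OnWidgetRemove and the construction script are empty.
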(event Custom|OnWidgetRemove)

(fn ConstructionScript)

(fn SwitchCurrentDevice
  (params (Key :type Key%20Structure :default "None"))
  (if (Class|KismetInputLibrary|KeyIsGamepadKey Key)
    (if (Utilities|Enum|Equal(Enum) (Variables|Default|GetCurrentDevice) "NewEnumerator0")
      (bind _output_get (Variables|Default|SetCurrentDevice "NewEnumerator1"))
      (Default|CallSwitchInputDevice _output_get))
    (elif (Utilities|Enum|Equal(Enum) (Variables|Default|GetCurrentDevice) "NewEnumerator1")
      (bind _output_get_2 (Variables|Default|SetCurrentDevice "NewEnumerator0"))
      (Default|CallSwitchInputDevice _output_get_2))))

(fn OnMouseMovement
  (bind (_locationx _locationy) (Game|Player|GetMousePosition))
  (bind _returnvalue (Class|GameUserSettings|GetDefaultResolution))
  (if (or (!= _locationx (Math|Conversions|ToFloat(Integer) (.X (Utilities|Struct|BreakIntPoint _returnvalue)))) (!= _locationy (Math|Conversions|ToFloat(Integer) (.Y (Utilities|Struct|BreakIntPoint _returnvalue)))))
    (if (Utilities|Enum|Equal(Enum) (Variables|Default|GetCurrentDevice) "NewEnumerator1")
      (Development|PrintString "MouseMoved")
      (CallFunction|SwitchCurrentDevice (LocalVariables|GetInterpretationKeyEventAsMouseEvent)))))