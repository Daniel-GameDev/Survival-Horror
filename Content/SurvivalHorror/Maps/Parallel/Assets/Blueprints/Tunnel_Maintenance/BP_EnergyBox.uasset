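; BP_EnergyBox is an energy box that powers on when a BP_EnergyCell is inserted into it.
; BeginPlay sets the initial on or off look from HasEnergyCell.
; The first cell to overlap the Box is destroyed, then CallGotEnergy fires and EnergyOn runs, without updating HasEnergyCell.
; EnergyOn and EnergyOff toggle the built-in cell's visibility, the light color and the indicator's glow material.
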(event OnComponentBeginOverlap(Box)
  (params (OverlappedComponent :type Primitive%20Component%20Object%20Reference) (OtherActor :type Actor%20Object%20Reference) (OtherComp :type Primitive%20Component%20Object%20Reference) (OtherBodyIndex :type Integer) (bFromSweep :type Boolean) (SweepResult :type Hit%20Result%20Structure%20%28by%20ref%29))
  (bind _asbp_energy_cell (Utilities|Casting|CastToBP_EnergyCell OtherActor))
  (Utilities|FlowControl|DoOnce false
    (:Completed
      (Actor|DestroyActor _asbp_energy_cell)
      (Default|CallGotEnergy)
      (CallFunction|Energyon))))

(event EventBeginPlay
  (if (Variables|Default|GetHasEnergyCell)
    (CallFunction|Energyon)
    (else
      (CallFunction|EnergyOff))))

(fn ConstructionScript)

(fn Energyon
  (Development|SetHiddeninGame (Variables|Default|GetEnergyCell) false false)
  (Rendering|Components|Light|SetLightColor (Variables|Default|GetPointLight1) (Variables|Default|GetEnableColor) true)
  (Rendering|Material|SetMaterial (Variables|Default|GetIndicator) 0 "/Game/SurvivalHorror/Maps/Parallel/Assets/Materials/M_Glow_Inst_Button.M_Glow_Inst_Button"))

(fn EnergyOff
  (Development|SetHiddeninGame (Variables|Default|GetEnergyCell) true true)
  (Rendering|Components|Light|SetLightColor (Variables|Default|GetPointLight1) (Variables|Default|GetDisableColor) true)
  (Rendering|Material|SetMaterial (Variables|Default|GetIndicator) 0 "/Game/SurvivalHorror/Maps/Parallel/Assets/Materials/M_Glow_Inst_Alert.M_Glow_Inst_Alert"))