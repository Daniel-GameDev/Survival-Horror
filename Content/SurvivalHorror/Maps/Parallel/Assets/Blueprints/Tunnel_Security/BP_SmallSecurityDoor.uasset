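; Small security door for a tunnel area that slides open and closed along its local X axis.
; OpenGate takes an Open, Close or Half command and plays or reverses a timeline, scaled to TimeToComplete, that lerps the door's position.
; Half overwrites the open distance with a random value before playing.
; When the timeline finishes, it toggles the open state and broadcasts it through DoorAction.
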(event EventBeginPlay
  (Components|Timeline|SetPlayRate (Variables|Default|GetOpenDoorTime) (/ 1.0 (Variables|Default|GetTimeToComplete))))

(event EventOpenGate
  (params (GatesAct :type EGatesAction%20Enum :default "NewEnumerator0"))
  (bind _door (Variables|Default|GetDoor))
  (bind _relativelocation (Variables|/Script/Engine.SceneComponent|GetRelativeLocation _door))
  (switch Utilities|FlowControl|Switch|SwitchonEGatesAction GatesAct
    (:NewEnumerator0
      (if (not (Variables|Default|GetGatesOpened))
        (bind _openning (Timeline|OpenDoorTime Play)
          (:Update
            (Transformation|SetRelativeLocation _door (Math|Vector|MakeVector (Math|Float|Lerp 0.0 (Variables|Default|GetOpenValue) _openning) (.y _relativelocation) (.z _relativelocation)) false false))
          (:Finished
            (if (Variables|Default|GetGatesOpened)
              (Variables|Default|SetGatesOpened false)
              (Variables|Default|SetGates%20State "NewEnumerator1")
              (else
                (Variables|Default|SetGatesOpened true)
                (Variables|Default|SetGates%20State "NewEnumerator0")))
            (Default|CallDoorAction (Variables|Default|GetGates%20State))))))
    (:NewEnumerator1
      (if (Variables|Default|GetGatesOpened)
        (Timeline|OpenDoorTime Reverse)))
    (:NewEnumerator2
      (if (not (Variables|Default|GetGatesOpened))
        (Variables|Default|SetOpenValue (Math|Random|RandomFloatinRange 7e+01 1.5e+02))
        (Timeline|OpenDoorTime Play)))))

(fn ConstructionScript)