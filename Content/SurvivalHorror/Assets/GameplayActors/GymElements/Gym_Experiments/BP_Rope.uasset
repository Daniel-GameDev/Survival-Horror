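; Hanging rope actor that pairs a simulated Cable component with a chain of capsule components along its length.
; Construction traces down to fit cable length above the floor, calling Destroy when too short, which only acts with a valid GameInstance.
; BeginPlay spawns a visible capsule per cable segment.
; Tick moves each to its particle's XY and segment's mid Z, orienting it along neighboring capsules with look-at rotations.
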(event Custom|Destroy
  (if (Utilities|IsValid (Game|GetGameInstance))
    (Actor|DestroyActor)))

(event EventBeginPlay
  (bind _cable (Variables|Default|GetCable))
  (bind _locations (Class|CableComponent|GetCableParticleLocations _cable))
  (for (_array_element _array_index) _locations
    (if (not (== _array_index (Utilities|Array|LastIndex _locations)))
      (bind _returnvalue (AddComponent|AddCapsuleComponent false (Math|Transform|MakeTransform _array_element "0, 0, 0" (Variables|Default|GetSocket_RelativeTransformScale))))
      (Utilities|Array|Add (Variables|Default|GetCapsuleArray) _returnvalue)
      (Development|SetHiddeninGame _returnvalue false false))))

(event EventTick
  (params (DeltaSeconds :type Float%20%28single-precision%29))
  (bind _cable (Variables|Default|GetCable))
  (bind _capsulearray (Variables|Default|GetCapsuleArray))
  (bind _locations (Class|CableComponent|GetCableParticleLocations _cable))
  (for (_array_element _array_index) _locations
    (if (not (== _array_index (Utilities|Array|LastIndex _locations)))
      (Transformation|SetWorldLocation (Utilities|Array|Get(acopy) _capsulearray _array_index) (Math|Vector|MakeVector (.X (Math|Vector|BreakVector _array_element)) (.Y (Math|Vector|BreakVector _array_element)) (/ (+ (.Z (Math|Vector|BreakVector _array_element)) (.Z (Math|Vector|BreakVector (Utilities|Array|Get(acopy) _locations (+ _array_index 1))))) 2.0)) false false)
      (Utilities|IsValid (Utilities|Array|Get(acopy) _capsulearray (+ _array_index 1))
        (:Is%20Valid
          (Transformation|SetWorldRotation (Utilities|Array|Get(acopy) _capsulearray _array_index) (Math|Rotator|MakeRotator 0.0 (+ (.pitch (Math|Rotator|FindLookatRotation (Transformation|GetWorldLocation (Utilities|Array|Get(acopy) _capsulearray _array_index)) (Transformation|GetWorldLocation (Utilities|Array|Get(acopy) _capsulearray (+ _array_index 1))))) 9e+01) (.yaw (Math|Rotator|FindLookatRotation (Transformation|GetWorldLocation (Utilities|Array|Get(acopy) _capsulearray _array_index)) (Transformation|GetWorldLocation (Utilities|Array|Get(acopy) _capsulearray (+ _array_index 1)))))) false false))
        (:Is%20Not%20Valid
          (Utilities|IsValid (Utilities|Array|Get(acopy) (Variables|Default|GetCapsuleArray) (- _array_index 1))
            (:Is%20Valid
              (Transformation|SetWorldRotation (Utilities|Array|Get(acopy) _capsulearray _array_index) (Math|Rotator|MakeRotator 0.0 (+ (.pitch (Math|Rotator|FindLookatRotation (Transformation|GetWorldLocation (Utilities|Array|Get(acopy) (Variables|Default|GetCapsuleArray) (- _array_index 1))) (Transformation|GetWorldLocation (Utilities|Array|Get(acopy) _capsulearray _array_index)))) 9e+01) (.yaw (Math|Rotator|FindLookatRotation (Transformation|GetWorldLocation (Utilities|Array|Get(acopy) (Variables|Default|GetCapsuleArray) (- _array_index 1))) (Transformation|GetWorldLocation (Utilities|Array|Get(acopy) _capsulearray _array_index))))) false false))))))))

(fn ConstructionScript
  (bind _cable (Variables|Default|GetCable))
  (bind _returnvalue (Transformation|GetWorldLocation _cable))
  (bind (_x _y _z) (Math|Vector|BreakVector _returnvalue))
  (bind (_outhit _returnvalue_2) (Collision|LineTraceByChannel _returnvalue (Math|Vector|MakeVector _x _y (- _z (Variables|Default|GetTraceCableLength))) "TraceTypeQuery1" false 0 "ForDuration" true "(R=1.000000,G=0.000000,B=0.000000,A=1.000000)" "(R=0.000000,G=1.000000,B=0.000000,A=1.000000)" 1e+01))
  (if _returnvalue_2
    (if (< (- (.Distance (Collision|BreakHitResult _outhit)) (Variables|Default|GetFloorSpacerLength)) 2e+02)
      (CallFunction|Destroy)
      (else
        (Variables|/Script/CableComponent.CableComponent|SetCableLength (Variables|Default|GetCable) (- (.Distance (Collision|BreakHitResult _outhit)) (Variables|Default|GetFloorSpacerLength)))))
    (else
      (Variables|/Script/CableComponent.CableComponent|SetCableLength (Variables|Default|GetCable) (- (Variables|Default|GetTraceCableLength) (Variables|Default|GetFloorSpacerLength))))))