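; Parent Blueprint for heavy draggable objects that the player interacts with through a "Carry" prompt.
; On BeginPlay, unless UseCustomSettings is set, it applies default focus and interaction settings (stencil, dot, icons, message, permanent use), then calls the parent BeginPlay.
; Interact reports the permanent-use flag and a fixed object type, and GetManipulateStatus exposes AllowManipulation.
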(event EventBeginPlay
  (bind _self self)
  ;[1 0 0] Check out Class Defaults
  (if (Variables|HeavySettings|GetUseCustomSettings)
    (|CallParentFunction :!label _label)
    (else
      (Utilities|FlowControl|Sequence
        (:then_0
          (Variables|/Game/SurvivalHorror/Assets/GameplayActors/GymElements/Common/BP_InteractableObject_Parent.BP_InteractableObject_Parent_C|SetStencilValue _self 0))
        (:then_1
          (Variables|/Game/SurvivalHorror/Assets/GameplayActors/GymElements/Common/BP_InteractableObject_Parent.BP_InteractableObject_Parent_C|SetDrawDotOnFocus _self false))
        (:then_2
          (Variables|/Game/SurvivalHorror/Assets/GameplayActors/GymElements/Common/BP_InteractableObject_Parent.BP_InteractableObject_Parent_C|SetInnerIcon _self "NewEnumerator3"))
        (:then_3
          (Variables|/Game/SurvivalHorror/Assets/GameplayActors/GymElements/Common/BP_InteractableObject_Parent.BP_InteractableObject_Parent_C|SetOuterIcon _self "NewEnumerator1"))
        (:then_4
          (Variables|/Game/SurvivalHorror/Assets/GameplayActors/GymElements/Common/BP_InteractableObject_Parent.BP_InteractableObject_Parent_C|SetPermanent%20Using _self true))
        (:then_5
          (Variables|/Game/SurvivalHorror/Assets/GameplayActors/GymElements/Common/BP_InteractableObject_Parent.BP_InteractableObject_Parent_C|SetMessage _self "Carry"))
        (:then_6
          (goto _label))))))

(event Collision|EventActorBeginOverlap
  (params (OtherActor :type Actor%20Object%20Reference))
  ;[1 0 0] Check out Class Defaults
)

(event EventTick
  (params (DeltaSeconds :type Float%20%28single-precision%29))
  ;[1 0 0] Check out Class Defaults
)

(fn ConstructionScript
  (|CallParentFunction))

(fn Interact
  (params (Interacter :type Primitive%20Component%20Object%20Reference) (Pawn :type BP%20First%20Person%20Char%20Object%20Reference))
  (return (Variables|Default|GetPermanent%20Using self) "NewEnumerator1"))

(fn GetManipulateStatus
  (return (Variables|HeavySettings|GetAllowManipulation)))