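; Player controller for the UMG_T1 menu test, which opens the player menu from the Menu_UMG_T1 input action.
; On press it creates a new WBP_PlayerMenu_UI_UMG_T1 widget, adds it to the viewport and switches to UI-only input focused on it.
; It checks whether the pressed key is a gamepad key and shows the mouse cursor only for non-gamepad input.
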(event Input|ActionEvents|InputActionMenu_UMG_T1
  (params (Key :type Key%20Structure :default "None"))
  (bind _self self)
  (:Pressed
    (if (Class|KismetInputLibrary|KeyIsGamepadKey Key)
      (bind _returnvalue (UserInterface|CreateWidget "/Game/SurvivalHorror/Maps/Menus/Tests/UMG_T1/UI/WBP_PlayerMenu_UI_UMG_T1.WBP_PlayerMenu_UI_UMG_T1_C" _self))
      (bind _output_get (Variables|Default|SetPlayerMenu _returnvalue))
      (UserInterface|Viewport|AddtoViewport _output_get 0)
      (Input|SetInputModeUIOnly self (Variables|Default|GetPlayerMenu) "DoNotLock")
      (else
        (bind _returnvalue_2 (UserInterface|CreateWidget "/Game/SurvivalHorror/Maps/Menus/Tests/UMG_T1/UI/WBP_PlayerMenu_UI_UMG_T1.WBP_PlayerMenu_UI_UMG_T1_C" _self))
        (bind _output_get_2 (Variables|Default|SetPlayerMenu _returnvalue_2))
        (UserInterface|Viewport|AddtoViewport _output_get_2 0)
        (Input|SetInputModeUIOnly self (Variables|Default|GetPlayerMenu) "DoNotLock")
        (Variables|Default|SetbShowMouseCursor true)))))

(fn ConstructionScript)