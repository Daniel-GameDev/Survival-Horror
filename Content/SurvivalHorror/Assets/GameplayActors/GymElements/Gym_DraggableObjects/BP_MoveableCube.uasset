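; BP_MoveableCube is a gym draggable object that the first-person character can push.
; Two trigger volumes, XAxisCollision and YAxisCollision, turn on the cube's physics simulation and set the character's Pushing flag on overlap.
; Leaving either volume turns physics off and clears the flag, without checking whether the other volume is still overlapped.
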(event OnComponentBeginOverlap(XAxisCollision)
  (params (OverlappedComponent :type Primitive%20Component%20Object%20Reference) (OtherActor :type Actor%20Object%20Reference) (OtherComp :type Primitive%20Component%20Object%20Reference) (OtherBodyIndex :type Integer) (bFromSweep :type Boolean) (SweepResult :type Hit%20Result%20Structure%20%28by%20ref%29))
  ;[1 1 1] X Axis Collision
  (bind _asbp_first_person_char (Utilities|Casting|CastToBP_FirstPerson_Char OtherActor))
  (Physics|SetSimulatePhysics (Variables|Default|GetCube) true)
  (Variables|/Game/SurvivalHorror/Assets/Characters/FirstPerson/Main/BP_FirstPerson_Char.BP_FirstPerson_Char_C|SetPushing _asbp_first_person_char true))

(event OnComponentEndOverlap(XAxisCollision)
  (params (OverlappedComponent :type Primitive%20Component%20Object%20Reference) (OtherActor :type Actor%20Object%20Reference) (OtherComp :type Primitive%20Component%20Object%20Reference) (OtherBodyIndex :type Integer))
  ;[1 1 1] X Axis Collision
  (bind _asbp_first_person_char (Utilities|Casting|CastToBP_FirstPerson_Char OtherActor))
  (Physics|SetSimulatePhysics (Variables|Default|GetCube) false)
  (Variables|/Game/SurvivalHorror/Assets/Characters/FirstPerson/Main/BP_FirstPerson_Char.BP_FirstPerson_Char_C|SetPushing _asbp_first_person_char false))

(event OnComponentBeginOverlap(YAxisCollision)
  (params (OverlappedComponent :type Primitive%20Component%20Object%20Reference) (OtherActor :type Actor%20Object%20Reference) (OtherComp :type Primitive%20Component%20Object%20Reference) (OtherBodyIndex :type Integer) (bFromSweep :type Boolean) (SweepResult :type Hit%20Result%20Structure%20%28by%20ref%29))
  ;[1 1 1] Y Axis Collision
  (bind _asbp_first_person_char (Utilities|Casting|CastToBP_FirstPerson_Char OtherActor))
  (Physics|SetSimulatePhysics (Variables|Default|GetCube) true)
  (Variables|/Game/SurvivalHorror/Assets/Characters/FirstPerson/Main/BP_FirstPerson_Char.BP_FirstPerson_Char_C|SetPushing _asbp_first_person_char true))

(event OnComponentEndOverlap(YAxisCollision)
  (params (OverlappedComponent :type Primitive%20Component%20Object%20Reference) (OtherActor :type Actor%20Object%20Reference) (OtherComp :type Primitive%20Component%20Object%20Reference) (OtherBodyIndex :type Integer))
  ;[1 1 1] Y Axis Collision
  (bind _asbp_first_person_char (Utilities|Casting|CastToBP_FirstPerson_Char OtherActor))
  (Physics|SetSimulatePhysics (Variables|Default|GetCube) false)
  (Variables|/Game/SurvivalHorror/Assets/Characters/FirstPerson/Main/BP_FirstPerson_Char.BP_FirstPerson_Char_C|SetPushing _asbp_first_person_char false))

(fn ConstructionScript)