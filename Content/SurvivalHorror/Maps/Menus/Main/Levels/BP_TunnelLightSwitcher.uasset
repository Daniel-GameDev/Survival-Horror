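; Main menu tunnel light switcher that puts the tunnel lighting into a red alert state.
; Its SwitchLight event gathers every BP_Tunnel_MainLight and BP_Tunnel_SpotLight actor in the level.
; It sets radius, intensity and red or red-orange color on their light components and swaps their meshes to an alert glow material.
; The switch is one-way, with no restore logic.
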(event Custom|SwitchLight
  (bind _outactors (Actor|GetAllActorsOfClass "/Game/SurvivalHorror/Maps/Parallel/Assets/Blueprints/Tunnel/BP_Tunnel_MainLight.BP_Tunnel_MainLight_C"))
  (Variables|Default|SetTunnelMainLight _outactors)
  (bind _outactors_2 (Actor|GetAllActorsOfClass "/Game/SurvivalHorror/Maps/Parallel/Assets/Blueprints/Tunnel/BP_Tunnel_SpotLight.BP_Tunnel_SpotLight_C"))
  (Variables|Default|SetTunnelSpotLight _outactors_2)
  (Utilities|FlowControl|Sequence
    (:then_0
      (for _array_element (Variables|Default|GetTunnelSpotLight)
        (Rendering|Lighting|SetAttenuationRadius (Variables|/Game/SurvivalHorror/Maps/Parallel/Assets/Blueprints/Tunnel/BP_Tunnel_SpotLight.BP_Tunnel_SpotLight_C|GetSpotLight _array_element) 6.5e+03)
        (Rendering|Components|Light|SetIntensity (Variables|/Game/SurvivalHorror/Maps/Parallel/Assets/Blueprints/Tunnel/BP_Tunnel_SpotLight.BP_Tunnel_SpotLight_C|GetSpotLight _array_element) 1.5e+04)
        (Rendering|Components|Light|SetLightColor (Variables|/Game/SurvivalHorror/Maps/Parallel/Assets/Blueprints/Tunnel/BP_Tunnel_SpotLight.BP_Tunnel_SpotLight_C|GetSpotLight _array_element) "(R=1.000000,G=0.103898,B=0.000000,A=1.000000)" true)
        (Rendering|Material|SetMaterial (Variables|/Game/SurvivalHorror/Maps/Parallel/Assets/Blueprints/Tunnel/BP_Tunnel_SpotLight.BP_Tunnel_SpotLight_C|GetStaticMesh _array_element) 0 "/Game/SurvivalHorror/Maps/Parallel/Assets/Materials/M_Glow_Inst_Alert.M_Glow_Inst_Alert")))
    (:then_1
      (for _array_element_2 (Variables|Default|GetTunnelMainLight)
        (Rendering|Lighting|SetAttenuationRadius (Variables|/Game/SurvivalHorror/Maps/Parallel/Assets/Blueprints/Tunnel/BP_Tunnel_MainLight.BP_Tunnel_MainLight_C|GetPointLight _array_element_2) 6.5e+03)
        (Rendering|Components|Light|SetIntensity (Variables|/Game/SurvivalHorror/Maps/Parallel/Assets/Blueprints/Tunnel/BP_Tunnel_MainLight.BP_Tunnel_MainLight_C|GetPointLight _array_element_2) 1.5e+04)
        (Rendering|Components|Light|SetLightColor (Variables|/Game/SurvivalHorror/Maps/Parallel/Assets/Blueprints/Tunnel/BP_Tunnel_MainLight.BP_Tunnel_MainLight_C|GetPointLight _array_element_2) "(R=1.000000,G=0.000000,B=0.000000,A=1.000000)" true)
        (Rendering|Material|SetMaterial (Variables|/Game/SurvivalHorror/Maps/Parallel/Assets/Blueprints/Tunnel/BP_Tunnel_MainLight.BP_Tunnel_MainLight_C|GetStaticMesh _array_element_2) 0 "/Game/SurvivalHorror/Maps/Parallel/Assets/Materials/M_Glow_Inst_Alert.M_Glow_Inst_Alert")))))

(fn ConstructionScript)