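; Item data component for the InvT1 gym inventory that lets its owning actor be picked up by a player.
; On BeginPlay it turns on replication for the owner.
; Interacting passes the ItemID row name and Quantity to the character's InventorySystemInvT1, destroying the owner only if everything is added.
; A partial add leaves the stored Quantity unchanged, and LookAt returns an empty string.
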(event EventBeginPlay
  (Networking|SetReplicates (Components|GetOwner) true))

(event EventInteractwith
  (params (FPChar :type BP%20First%20Person%20Char%20Object%20Reference))
  (bind _inventorysystem_invt1 (Variables|/Game/SurvivalHorror/Assets/Characters/FirstPerson/Main/BP_FirstPerson_Char.BP_FirstPerson_Char_C|GetInventorySystem_InvT1 FPChar))
  (Utilities|IsValid _inventorysystem_invt1
    (:Is%20Valid
      (bind (_success _quantityremaining) (Default|AddtoInventory _inventorysystem_invt1 (.rowname (Variables|Default|GetItemID)) (Variables|Default|GetQuantity)))
      (if (and (Math|Boolean|Equal(Boolean) _success true) (== _quantityremaining 0))
        (Actor|DestroyActor (Components|GetOwner))))))

(fn Lookat
  (return ""))