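; Interactable tunnel security button for a linked gate, which starts active, disabled or broken according to ButtonState, shown through glow material and spotlight.
; Interacting toggles GatesAct between open and close, calls Pressed and runs a timeline that slides the button.
; A DoOnce blocks further presses until the bound Door event reports open or closed, restoring the active color.
; A half-open report instead swaps in a plain material and destroys the light.
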(event Custom|DoorOpened_Event_0
  (params (GatesState :type EGatesAction%20Enum :default "NewEnumerator0"))
  (bind _button (Variables|Default|GetButton))
  (bind _relativelocation (Variables|/Script/Engine.SceneComponent|GetRelativeLocation _button))
  (switch Utilities|FlowControl|Switch|SwitchonEGatesAction GatesState
    (:NewEnumerator0
      (Development|PrintString (Utilities|String|EnumtoString GatesState) :!label _label)
      (Utilities|FlowControl|Sequence
        (:then_0
          (Rendering|Material|SetVectorParameterValue (Variables|Default|GetButtonMaterial) "GlowTint" (Variables|Default|GetActiveColor) :!class /Script/Engine.MaterialInstanceDynamic)
          (Rendering|Components|Light|SetLightColor (Variables|Default|GetSpotLight) (Variables|Default|GetActiveColor) true))
        (:then_1
          (Utilities|FlowControl|DoOnce (Variables|Default|GetDisableButton%28Temp-NeedToUpdatedInteractbleObject%29)) ; enters at Reset
        )))
    (:NewEnumerator1
      (goto _label))
    (:NewEnumerator2
      (Rendering|Material|SetMaterial (Variables|Default|GetButton) 0 "/Engine/BasicShapes/BasicShapeMaterial.BasicShapeMaterial")
      (Components|DestroyComponent (Variables|Default|GetSpotLight)))))

(event EventInteracting
  (params (Interacter :type Pawn%20Object%20Reference))
  (bind _button (Variables|Default|GetButton))
  (bind _relativelocation (Variables|/Script/Engine.SceneComponent|GetRelativeLocation _button))
  (Utilities|FlowControl|DoOnce (Variables|Default|GetDisableButton%28Temp-NeedToUpdatedInteractbleObject%29)
    (:Completed
      (Utilities|FlowControl|FlipFlop
        (:A
          (Variables|Default|SetGates%20Act "NewEnumerator0"))
        (:B
          (Variables|Default|SetGates%20Act "NewEnumerator1")))
      (Default|CallPressed)
      (switch Utilities|FlowControl|Switch|SwitchonEGatesAction (Variables|Default|GetGates%20Act)
        (:NewEnumerator0
          (bind _pressing (Timeline|ButtonPressTime Play)
            (:Update
              (Transformation|SetRelativeLocation _button (Math|Vector|MakeVector (Math|Float|Lerp -8e+01 -83.0 _pressing) (.y _relativelocation) (.z _relativelocation)) false false))
            (:Finished
              (Utilities|FlowControl|Sequence
                (:then_0
                  (Rendering|Material|SetVectorParameterValue (Variables|Default|GetButtonMaterial) "GlowTint" (Variables|Default|GetDisableColor) :!class /Script/Engine.MaterialInstanceDynamic)
                  (Rendering|Components|Light|SetLightColor (Variables|Default|GetSpotLight) (Variables|Default|GetDisableColor) true))
                (:then_1)))))
        (:NewEnumerator1
          (Timeline|ButtonPressTime Reverse))))))

(event EventBeginPlay
  (|CallParentFunction)
  (EventDispatchers|AssignDoorAction (Variables|Default|GetDoor) (EventDispatchers|CreateEvent :!event Custom|DoorOpened_Event_0))
  (switch Utilities|FlowControl|Switch|SwitchonEButtonState (Variables|Default|GetButtonState)
    (:NewEnumerator0
      (Variables|Default|SetDisableButton%28Temp-NeedToUpdatedInteractbleObject%29 false))
    (:NewEnumerator1
      (Variables|Default|SetDisableButton%28Temp-NeedToUpdatedInteractbleObject%29 true)
      (Rendering|Material|SetVectorParameterValue (Variables|Default|GetButtonMaterial) "GlowTint" (Variables|Default|GetDisableColor) :!class /Script/Engine.MaterialInstanceDynamic)
      (Rendering|Components|Light|SetLightColor (Variables|Default|GetSpotLight) (Variables|Default|GetDisableColor) true))
    (:NewEnumerator2
      (Variables|Default|SetDisableButton%28Temp-NeedToUpdatedInteractbleObject%29 true)
      (Rendering|Material|SetMaterial (Variables|Default|GetButton) 0 "/Engine/BasicShapes/BasicShapeMaterial.BasicShapeMaterial")
      (Components|DestroyComponent (Variables|Default|GetSpotLight)))))

(fn ConstructionScript
  (bind _returnvalue (Rendering|Material|CreateDynamicMaterialInstance (Variables|Default|GetButton) 0 "/Game/SurvivalHorror/Maps/Parallel/Assets/Materials/M_Glow_Inst_Button.M_Glow_Inst_Button" "None" :!class /Script/Engine.PrimitiveComponent))
  (Variables|Default|SetButtonMaterial _returnvalue)
  (switch Utilities|FlowControl|Switch|SwitchonEButtonState (Variables|Default|GetButtonState)
    (:NewEnumerator0
      (Rendering|Material|SetVectorParameterValue (Variables|Default|GetButtonMaterial) "GlowTint" (Variables|Default|GetActiveColor) :!class /Script/Engine.MaterialInstanceDynamic)
      (Rendering|Components|Light|SetLightColor (Variables|Default|GetSpotLight) (Variables|Default|GetActiveColor) true))
    (:NewEnumerator1
      (Rendering|Material|SetVectorParameterValue (Variables|Default|GetButtonMaterial) "GlowTint" (Variables|Default|GetDisableColor) :!class /Script/Engine.MaterialInstanceDynamic)
      (Rendering|Components|Light|SetLightColor (Variables|Default|GetSpotLight) (Variables|Default|GetDisableColor) true))))