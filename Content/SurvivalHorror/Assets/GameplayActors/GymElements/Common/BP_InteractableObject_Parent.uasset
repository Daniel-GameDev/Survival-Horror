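; Parent Blueprint for interactable gym objects, built from a static mesh, inner and outer detection spheres and a billboard widget for each range.
; BeginPlay sends icons to both widgets through a widget interface, applies the mesh's stencil value and optionally shows the spheres for debugging.
; Interactors query focus settings, toggle either billboard and test inner-sphere overlap.
; Interact only returns PermanentUsing; the Interacting event is empty and unconnected.
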(event Custom|Interacting)

(event EventBeginPlay
  (bind _innerbillboardwidget (Variables|Default|GetInnerBillBoardWidget))
  (bind _outerbillboardwidget (Variables|Default|GetOuterBillBoardWidget))
  (bind _returnvalue (UserInterface|GetWidget _innerbillboardwidget))
  (bind _returnvalue_2 (UserInterface|GetWidget _outerbillboardwidget))
  (Utilities|FlowControl|Sequence
    (:then_0
      (if (Utilities|DoesObjectImplementInterface _returnvalue_2 "/Game/SurvivalHorror/Assets/GameplayActors/GymElements/Common/Interfaces/BPI_WidgetInteractionObjectType.BPI_WidgetInteractionObjectType_C")
        (Class|BPIWidgetInteractionObjectType|SetIcon(Message) _returnvalue_2 (Variables|InteractableSettings|GetOuterIcon))))
    (:then_1
      (if (Utilities|DoesObjectImplementInterface _returnvalue "/Game/SurvivalHorror/Assets/GameplayActors/GymElements/Common/Interfaces/BPI_WidgetInteractionObjectType.BPI_WidgetInteractionObjectType_C")
        (Class|BPIWidgetInteractionObjectType|SetIcon(Message) _returnvalue (Variables|InteractableSettings|GetInnerIcon))))
    (:then_2
      ;[1 1 1] Part of Consttruction Script > Set this value by choosing type of object (using tag?)
      (Rendering|SetCustomDepthStencilValue (Variables|Default|GetStaticMesh) (Variables|InteractableSettings|GetStencilValue)))
    (:then_3
      (if (Variables|Debug|GetShowCollisionSpheres)
        (Development|SetHiddeninGame (Variables|Default|GetOuterSphere) false false)
        (Development|SetHiddeninGame (Variables|Default|GetInnerSphere) false false)
        (else
          (Development|SetHiddeninGame (Variables|Default|GetOuterSphere) true false)
          (Development|SetHiddeninGame (Variables|Default|GetInnerSphere) true false))))))

(event EventSetBillboardVisibility
  (params (Inner%281%29/Outer%280%29 :type Boolean) (Visible :type Boolean))
  (if Inner%281%29/Outer%280%29
    (Rendering|SetVisibility (Variables|Default|GetInnerBillBoardWidget) Visible false)
    (else
      (Rendering|SetVisibility (Variables|Default|GetOuterBillBoardWidget) Visible false))))

(fn ConstructionScript)

(fn GetSettings
  (return (Variables|InteractableSettings|GetDrawDotOnFocus) (!= (Variables|InteractableSettings|GetStencilValue) 0) (Variables|InteractableSettings|GetMessage)))

(fn Interact
  (params (Interacter :type Primitive%20Component%20Object%20Reference))
  (return (Variables|InteractableSettings|GetPermanent%20Using)))

(fn RequestCollisionType
  (params (Interapter :type Capsule%20Component%20Object%20Reference))
  (LocalVariables|SetInnerValue (Utilities|Array|ContainsItem (Class|PrimitiveComponent|GetOverlappingComponents (Variables|Default|GetInnerSphere)) Interapter))
  (return (LocalVariables|GetInnerValue)))